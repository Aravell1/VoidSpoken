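; Player controller for the title screen, which plays an intro video and then shows the title menu.
; On BeginPlay it shows the cursor, blocks look and move input, adds the video widget and starts a media sound component.
; Pressing any key while the media sound plays triggers ShowTitlescreen once, which stops the sound, creates the title screen widget and focuses it in Game and UI input mode.
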(event Custom|Show%20Titlescreen
  ;[1 1 1] Create/Show Title Screen
  (Audio|Components|Audio|Stop (Variables|Default|GetMediaSound))
  (bind _returnvalue (UserInterface|CreateWidget "/Game/User_Interface/Titlescreen/Blueprints/UI_Titlescreen.UI_Titlescreen_C" self))
  (UserInterface|Viewport|AddtoViewport _returnvalue 0)
  (Input|SetInputModeGameandUI self _returnvalue "DoNotLock" false))

(event EventBeginPlay
  ;[1 1 1] Set Up
  (Variables|Default|SetbShowMouseCursor true)
  (Input|SetIgnoreLookInput true)
  (Input|SetIgnoreMoveInput true)
  (bind _returnvalue (UserInterface|CreateWidget "/Game/User_Interface/Titlescreen/Blueprints/UI_TitlescreenVideo.UI_TitlescreenVideo_C" self))
  (UserInterface|Viewport|AddtoViewport _returnvalue 0)
  (CameraShake|Start (Variables|Default|GetMediaSound)))

(event Input|KeyboardEvents|AnyKey
  (params (Key :type Key%20Structure :default "None"))
  ;[1 1 1] Skipping Intro Video Logic
  (:Pressed
    (if (Audio|Components|Audio|IsPlaying (Variables|Default|GetMediaSound))
      (Utilities|FlowControl|DoOnce false
        (:Completed
          (CallFunction|ShowTitlescreen))))))

(fn ConstructionScript)