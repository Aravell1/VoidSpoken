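; PC_TitlescreenController is the player controller for the title screen, setting up its UI and audio.
; On BeginPlay it shows the mouse cursor, ignores look and move input, adds a video widget to the viewport and starts a media sound component.
; After a short delay it adds the title screen widget on top and switches to Game and UI input mode focused on that widget.
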(event EventBeginPlay
  (Variables|Default|SetbShowMouseCursor true)
  (Input|SetIgnoreLookInput true)
  (Input|SetIgnoreMoveInput true)
  (bind _returnvalue (UserInterface|CreateWidget "/Game/User_Interface/UI_TitlescreenVideo.UI_TitlescreenVideo_C" self))
  (UserInterface|Viewport|AddtoViewport _returnvalue 0)
  (CameraShake|Start (Variables|Default|GetMediaSound))
  (Utilities|FlowControl|Delay 2.0)
  (bind _returnvalue_2 (UserInterface|CreateWidget "/Game/User_Interface/UI_Titlescreen.UI_Titlescreen_C" self))
  (UserInterface|Viewport|AddtoViewport _returnvalue_2 0)
  (Input|SetInputModeGameandUI self _returnvalue_2 "DoNotLock" false))

(fn ConstructionScript)