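; A test weapon Blueprint that equips itself to the first player character when play begins.
; On BeginPlay it calls Equip on that character, then casts it to BaseEntity and sets itself as that entity's EquippedWeapon.
; If the EquippedCharacter mesh has a "Weapon Point" socket, the weapon attaches there, snapping location, rotation and scale.
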(event EventBeginPlay
  (bind _returnvalue (Game|GetPlayerCharacter 0))
  (bind _equippedcharacter (Variables|Default|GetEquippedCharacter))
  (bind _mesh (Variables|/Script/Engine.Character|GetMesh _equippedcharacter))
  (Class|BaseWeapon|Equip self _returnvalue)
  (bind _asbase_entity (Utilities|Casting|CastToBaseEntity _returnvalue))
  (bind _output_get (Variables|/Script/VoidSpoken.PlayerCharacter|SetEquippedWeapon _asbase_entity self))
  (if (Transformation|DoesSocketExist _mesh "Weapon Point")
    (Transformation|AttachComponentToComponent _output_get _mesh "Weapon Point" "SnapToTarget" "SnapToTarget" "SnapToTarget" false)))

(fn ConstructionScript)