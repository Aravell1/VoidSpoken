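; PortalSpawn_BP is a portal spawn actor that sends Gatekeeper-spawned enemies after the player when an attack order fires.
; On BeginPlay it binds its OrderAttack event to the OrderAttackBP dispatcher.
; That event loops through the game mode's GatekeeperEnemySpawns, disables each enemy's CanReset and calls SeePlayer on any not already targeting the player character.
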(event Custom|OrderAttack
  (bind _returnvalue (Game|GetPlayerCharacter 0))
  (bind _asvoid_spoken_game_mode_bp (Utilities|Casting|CastToVoidSpoken_GameMode_BP (Game|GetGameMode)))
  (for _array_element (Variables|/Script/VoidSpoken.VoidSpokenGameModeBase|GetGatekeeperEnemySpawns _asvoid_spoken_game_mode_bp)
    (bind _asbase_enemy_bp (Utilities|Casting|CastToBaseEnemy_BP _array_element))
    (Variables|/Game/Blueprints/Enemies/BaseEnemy_BP.BaseEnemy_BP_C|SetCanReset _asbase_enemy_bp false)
    (if (not (== (Variables|/Game/Blueprints/Enemies/BaseEnemy_BP.BaseEnemy_BP_C|GetAttackTarget _asbase_enemy_bp) _returnvalue))
      (Default|SeePlayer _asbase_enemy_bp _returnvalue))))

(event EventBeginPlay
  (EventDispatchers|AssignOrderAttackBP (delegate Custom|OrderAttack)))

(fn ConstructionScript)