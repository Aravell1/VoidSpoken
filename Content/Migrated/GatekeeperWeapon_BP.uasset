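; Gatekeeper weapon Blueprint that equips itself to the Gatekeeper characters in the level.
; On BeginPlay it loops over every Gatekeeper actor, calls Equip with that character's attack as damage, and links weapon and character to each other.
; It then attaches to the character mesh's WeaponSocket if present, so the single weapon is reassigned on each iteration.
; The graph is marked for a switch to C++.
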(event EventBeginPlay
  ;[1 1 1] Switch to C++
  (bind _outactors (Actor|GetAllActorsOfClass "/Script/VoidSpoken.Gatekeeper"))
  (for _array_element _outactors
    (bind _returnvalue (Class|BaseEnemy|GetAttack _array_element))
    (Class|EnemyWeapon|Equip self _array_element _returnvalue)
    (Variables|Default|SetEquippedCharacter _array_element)
    (Variables|/Script/VoidSpoken.BaseEnemy|SetEquippedWeapon _array_element self)
    (if (Transformation|DoesSocketExist (Variables|/Script/Engine.Character|GetMesh (Variables|Default|GetEquippedCharacter)) "WeaponSocket")
      (Transformation|AttachComponentToComponent (Variables|/Script/Engine.Character|GetMesh (Variables|Default|GetEquippedCharacter)) "WeaponSocket" "KeepRelative" "KeepRelative" "KeepRelative" false))))

(fn ConstructionScript)