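; Gatekeeper boss character that shows an on-screen health bar and can be locked onto by a targeting system.
; PawnSensing creates the boss health bar widget on every sighting, with no guard against duplicates.
; A bound update event refreshes the bar from Stats and removes it when health reaches zero.
; TargetingComponent initializes on the Spine bone at BeginPlay, and query functions expose it and the IsDead flag.
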(event OnSeePawn(PawnSensing)
  (params (Pawn :type Pawn%20Object%20Reference))
  (bind _stats (Variables|Default|GetStats))
  (bind _returnvalue (UserInterface|CreateWidget "/Game/Blueprints/Bosses/BossHealthBarWidget.BossHealthBarWidget_C"))
  (bind _output_get (Variables|Default|SetHealthBar _returnvalue))
  (UserInterface|Viewport|AddtoViewport _output_get 0)
  (Default|HealthUpdate (Variables|Default|GetHealthBar) (Variables|/Script/VoidSpoken.StatsMasterClass|GetHealth _stats) (Class|StatsMasterClass|GetMaxHealth _stats)))

(event Custom|UpdateHPBar
  (bind _healthbar (Variables|Default|GetHealthBar))
  (bind _stats (Variables|Default|GetStats))
  (bind _health (Variables|/Script/VoidSpoken.StatsMasterClass|GetHealth _stats))
  (if (> _health 0.0)
    (Default|HealthUpdate _healthbar _health (Class|StatsMasterClass|GetMaxHealth _stats))
    (else
      (Widget|RemovefromParent _healthbar))))

(event EventBeginPlay
  (bind _self self)
  (EventDispatchers|BindEventtoUpdateHealthBar (delegate Custom|UpdateHPBar))
  ;[0 0 0] Initialize Enemy Targeting
  (Default|Initialization (Variables|Default|GetTargetingComponent) _self (Pawn|GetController _self) (Variables|Character|GetMesh) "Spine"))

(fn ConstructionScript)

(fn TargetDeadInformation
  (return (Variables|Default|GetbIsDead)))

(fn TargetInformations
  (return (Variables|Default|GetTargetingComponent)))