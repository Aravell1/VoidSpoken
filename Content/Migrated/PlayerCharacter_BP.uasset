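; Player character Blueprint that creates the HUD and compass bar, opens pause and inventory menus, and exposes normalized stats.
; TargetingComponent handles lock-on and target swapping, and filters mouse look input.
; An overlap volume collects tagged interest components, and C spawns a Niagara ring with beams toward each, throttled by an AntiSpam macro.
; Use triggers the focus consumable, and temporary debug inputs test damage and the loading screen.
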(event OnComponentBeginOverlap(CompassInterest)
  (params (OverlappedComponent :type Primitive%20Component%20Object%20Reference) (OtherActor :type Actor%20Object%20Reference) (OtherComp :type Primitive%20Component%20Object%20Reference) (OtherBodyIndex :type Integer) (bFromSweep :type Boolean) (SweepResult :type Hit%20Result%20Structure%20%28by%20ref%29))
  ;[1 0.1451 0.8144] Compass System
  ;;[1 1 1] Adding the "interest" to the array
  (if (Actor|ActorHasTag OtherActor "Compass Interest")
    (Utilities|Array|Add (Variables|Default|GetCompass%20Interest%20Array) (Utilities|ResolveSoftReference OtherComp))
    (Development|PrintString (Utilities|GetDisplayName OtherComp))))

(event OnComponentEndOverlap(CompassInterest)
  (params (OverlappedComponent :type Primitive%20Component%20Object%20Reference) (OtherActor :type Actor%20Object%20Reference) (OtherComp :type Primitive%20Component%20Object%20Reference) (OtherBodyIndex :type Integer))
  ;[1 0.1451 0.8144] Compass System
  ;;[1 1 1] Removing "Interest" from Array
  (Utilities|Array|RemoveItem (Variables|Default|GetCompass%20Interest%20Array) (Utilities|ResolveSoftReference OtherComp)))

(event Custom|CreateHUD
  (bind _returnvalue (UserInterface|CreateWidget "/Game/Blueprints/Player/Compass/wdg_compassBar.wdg_compassBar_C"))
  (bind _returnvalue_2 (UserInterface|CreateWidget "/Game/User_Interface/HUD/Blueprints/UI_HUD.UI_HUD_C" (.AsPlayer%20Controller (Utilities|Casting|CastToPlayerController (Pawn|GetController)))))
  (UserInterface|Viewport|AddtoViewport _returnvalue_2 0))

(event EventBeginPlay
  (bind _self self)
  (CallFunction|CreateHUD)
  ;[0 0 0] Initialize Player Targeting
  (|CallParentFunction)
  (Default|Initialization (Variables|Default|GetTargetingComponent) _self (Pawn|GetController _self) (Variables|Character|GetMesh) "Spine2"))

(event Input|ActionEvents|InputActionTabTarget
  (params (Key :type Key%20Structure))
  ;[0 0 0] Targeting Inputs
  (:Pressed
    (Default|SwapTarget (Variables|Default|GetTargetingComponent))))

(event Input|ActionEvents|InputActionDamageTestBoss
  (params (Key :type Key%20Structure))
  (:Pressed
    (bind _outactors (Actor|GetAllActorsOfClass "/Game/Blueprints/Bosses/BaseBoss_BP.BaseBoss_BP_C"))
    (for _array_element _outactors
      (Default|DamageTest _array_element))))

(event Input|ActionEvents|InputActionInventory
  (params (Key :type Key%20Structure))
  (bind _returnvalue (Game|GetPlayerController 0))
  (:Pressed
    (if (not (Game|IsGamePaused))
      (Game|SetGamePaused true)
      (bind _returnvalue_2 (UserInterface|CreateWidget "/Game/User_Interface/HUD/Inventory.Inventory_C" _returnvalue))
      (UserInterface|Viewport|AddtoViewport _returnvalue_2 0)
      (Variables|/Script/Engine.PlayerController|SetbShowMouseCursor _returnvalue true))))

(event Input|ActionEvents|InputActionPause
  (params (Key :type Key%20Structure))
  (bind _returnvalue (Game|GetPlayerController 0))
  (:Pressed
    (if (not (Game|IsGamePaused))
      (Game|SetGamePaused true)
      (bind _returnvalue_2 (UserInterface|CreateWidget "/Game/User_Interface/HUD/Pause.Pause_C" _returnvalue))
      (UserInterface|Viewport|AddtoViewport _returnvalue_2 0)
      (Variables|/Script/Engine.PlayerController|SetbShowMouseCursor _returnvalue true))))

(event Input|ActionEvents|InputActionDamageTest
  (params (Key :type Key%20Structure))
  (:Pressed
    (bind _outactors (Actor|GetAllActorsOfClass "/Game/Blueprints/Enemies/BaseEnemy_BP.BaseEnemy_BP_C"))
    (for _array_element _outactors
      (Default|DamageTest _array_element))))

(event Input|ActionEvents|InputActionUse
  (params (Key :type Key%20Structure))
  (:Pressed
    (Class|PlayerCharacter|UseFocusConsumable (.AsPlayer%20Character%20BP (Utilities|Casting|CastToPlayerCharacter_BP (Game|Player|GetPlayerPawn 0))))))

(event Input|AxisEvents|InputAxisTurn/Mouse
  (params (AxisValue :type Float%20%28single-precision%29))
  ;[0 0 0] Targeting Inputs
  (Pawn|Input|AddControllerYawInput (Default|AxisTurn (Variables|Default|GetTargetingComponent) AxisValue)))

(event Input|AxisEvents|InputAxisLookup/downMouse
  (params (AxisValue :type Float%20%28single-precision%29))
  ;[0 0 0] Targeting Inputs
  (Pawn|Input|AddControllerPitchInput (Default|AxisLookUp (Variables|Default|GetTargetingComponent) AxisValue)))

(event Input|MouseEvents|MiddleMouseButton
  (params (Key :type Key%20Structure))
  ;[0 0 0] Targeting Inputs
  (:Pressed
    (Default|Lockon (Variables|Default|GetTargetingComponent))))

(event Input|KeyboardEvents|C
  (params (Key :type Key%20Structure))
  (bind _mesh (Variables|Character|GetMesh))
  (bind _returnvalue (Transformation|GetWorldLocation _mesh))
  ;[1 0.1451 0.8144] Compass System
  (:Pressed
    (Utilities|AntiSpam 1.0
      (:SpamFree
        (Niagara|SpawnSystematLocation "/Game/Migrated/NPS_CompassRing.NPS_CompassRing" (+ (Transformation|GetWorldLocation (Variables|Character|GetMesh)) "0,0,100.000000"))
        (for _array_element (Variables|Default|GetCompass%20Interest%20Array)
          (bind _returnvalue_2 (Niagara|SpawnSystematLocation "/Game/Migrated/NPS_CompassBeam.NPS_CompassBeam" (+ _returnvalue (* (Math|Vector|GetUnitDirection(Vector) _returnvalue (Transformation|GetWorldLocation (Utilities|ResolveSoftReference _array_element))) "1.000000,1.000000,0.000000" 1e+02) "0,0,100.000000")))
          (Niagara|SetNiagaraVariable(Vector3) _returnvalue_2 "User.Direction" (* (Math|Vector|GetUnitDirection(Vector) (+ _returnvalue (* (Math|Vector|GetUnitDirection(Vector) _returnvalue (Transformation|GetWorldLocation (Utilities|ResolveSoftReference _array_element))) "1.000000,1.000000,0.000000" 1e+02) "0,0,100.000000") (Transformation|GetWorldLocation (Utilities|ResolveSoftReference _array_element))) 25)))))))

(event Input|KeyboardEvents|Add
  (params (Key :type Key%20Structure))
  (bind _stats (Variables|Default|GetStats))
  ;[1 1 1] TO BE RREMOVED
  (:Pressed
    (Variables|/Script/VoidSpoken.StatsMasterClass|SetHealth _stats (- (Variables|/Script/VoidSpoken.StatsMasterClass|GetHealth _stats) 1e+01))))

(event Input|KeyboardEvents|L
  (params (Key :type Key%20Structure))
  ;[1 1 1] TO BE REMOVED - Loading Screen
  (:Pressed
    (bind _returnvalue (UserInterface|CreateWidget "/Game/User_Interface/LoadingScreen/Blueprints/UI_LoadingScreen.UI_LoadingScreen_C" (Game|GetPlayerController 0)))
    (bind _output_get (Variables|Default|SetLoading%20Screen _returnvalue))
    (UserInterface|Viewport|AddtoViewport _output_get 0))
  (:Released
    (Widget|RemovefromParent (Variables|Default|GetLoading%20Screen))))

(fn ConstructionScript)

(fn GetNormalizedFocus
  (bind _stats (Variables|Default|GetStats))
  (return (/ (Variables|/Script/VoidSpoken.StatsMasterClass|GetFocusPoints _stats) (Class|StatsMasterClass|GetMaxFocus _stats))))

(fn GetNormalizedHealth
  (bind _stats (Variables|Default|GetStats))
  (return (/ (Variables|/Script/VoidSpoken.StatsMasterClass|GetHealth _stats) (Class|StatsMasterClass|GetMaxHealth _stats))))

(fn GetNormalizedStamina
  (bind _stats (Variables|Default|GetStats))
  (return (/ (Variables|/Script/VoidSpoken.StatsMasterClass|GetStamina _stats) (Class|StatsMasterClass|GetMaxStamina _stats))))

(fn TargetDeadInformation
  (return false))

(fn TargetInformations
  (return (Variables|Default|GetTargetingComponent)))