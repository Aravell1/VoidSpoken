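; VoidSpoken game mode that handles player data saving and consumable item selection and use.
; BeginPlay caches the game instance, which InitializePlayerSavedData uses to gather player data and write it to a save slot.
; TabTarget cycles CurrentItem through the ItemTypes class array with a wrapping index.
; Three separate Use input events compare that class to health, focus and stamina pickups to trigger the matching consumable, with debug prints throughout.
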(event Custom|InitializePlayerSavedData
  (bind _gameinstanceref (Variables|Default|GetGameInstanceRef))
  (bind _savedgamename (Variables|/Game/Blueprints/SavingAndLoading/VoidSpokenGameInstance.VoidSpokenGameInstance_C|GetSavedGameName _gameinstanceref))
  (Default|SavePlayerData _gameinstanceref)
  (bind _returnvalue (SaveGame|SaveGametoSlot (Variables|/Game/Blueprints/SavingAndLoading/VoidSpokenGameInstance.VoidSpokenGameInstance_C|GetSaveGameData _gameinstanceref) _savedgamename))
  (if _returnvalue
    (Development|PrintString (Utilities|String|Append _savedgamename "?????????????"))
    (else
      (Development|PrintString "Saved Failed"))))

(event EventBeginPlay
  (bind _asvoid_spoken_game_instance (Utilities|Casting|CastToVoidSpokenGameInstance (Game|GetGameInstance)))
  (Variables|Default|SetGameInstanceRef _asvoid_spoken_game_instance))

(event EventTick
  (params (DeltaSeconds :type Float%20%28single-precision%29)))

(event Input|ActionEvents|InputActionUse
  (params (Key :type Key%20Structure :default "None"))
  (:Pressed
    (if (== "/Script/VoidSpoken.StaminaPickup" (Variables|VoidSpoken_GameMode_BP_C|GetCurrent%20Item (.AsVoid%20Spoken%20Game%20Mode%20BP (Utilities|Casting|CastToVoidSpoken_GameMode_BP (Game|GetGameMode)))))
      (Class|PlayerCharacter|UseStaminaConsumable)
      (Development|PrintString "Stamina Used"))))

(event Input|ActionEvents|InputActionTabTarget
  (params (Key :type Key%20Structure :default "None"))
  (bind _returnvalue (Game|GetGameMode))
  (bind _asvoid_spoken_game_mode_bp (Utilities|Casting|CastToVoidSpoken_GameMode_BP _returnvalue))
  (bind _itemtypes (Variables|/Script/VoidSpoken.VoidSpokenGameModeBase|GetItemTypes _asvoid_spoken_game_mode_bp))
  (:Pressed
    (bind _result (Math|Integer|IncrementInt (Variables|/Script/VoidSpoken.VoidSpokenGameModeBase|GetItemTypeIndex _asvoid_spoken_game_mode_bp))
      (:%20%20
        (bind _output_get (Variables|/Script/VoidSpoken.VoidSpokenGameModeBase|SetItemTypeIndex (.AsVoid%20Spoken%20Game%20Mode%20BP (Utilities|Casting|CastToVoidSpoken_GameMode_BP (Game|GetGameMode))) (Math|Integer|%(Integer) _result (Utilities|Array|Length _itemtypes))))
        (bind _output_get_2 (Variables|VoidSpoken_GameMode_BP_C|SetCurrent%20Item (.AsVoid%20Spoken%20Game%20Mode%20BP (Utilities|Casting|CastToVoidSpoken_GameMode_BP (Game|GetGameMode))) (Utilities|Array|Get(acopy) _itemtypes _output_get)))
        (Development|PrintString (Utilities|GetClassDisplayName _output_get_2))
        (if (not (== "/Script/VoidSpoken.HealthPickup" (Variables|VoidSpoken_GameMode_BP_C|GetCurrent%20Item (.AsVoid%20Spoken%20Game%20Mode%20BP (Utilities|Casting|CastToVoidSpoken_GameMode_BP (Game|GetGameMode))))))
          (if (not (== "/Script/VoidSpoken.FocusPickup" (Variables|VoidSpoken_GameMode_BP_C|GetCurrent%20Item (.AsVoid%20Spoken%20Game%20Mode%20BP (Utilities|Casting|CastToVoidSpoken_GameMode_BP (Game|GetGameMode))))))
            (if (== "/Script/VoidSpoken.StaminaPickup" (Variables|VoidSpoken_GameMode_BP_C|GetCurrent%20Item (.AsVoid%20Spoken%20Game%20Mode%20BP (Utilities|Casting|CastToVoidSpoken_GameMode_BP (Game|GetGameMode)))))
              _)))))))

(event Input|ActionEvents|InputActionUse
  (params (Key :type Key%20Structure :default "None"))
  (:Pressed
    (if (== "/Script/VoidSpoken.FocusPickup" (Variables|VoidSpoken_GameMode_BP_C|GetCurrent%20Item (.AsVoid%20Spoken%20Game%20Mode%20BP (Utilities|Casting|CastToVoidSpoken_GameMode_BP (Game|GetGameMode)))))
      (Class|PlayerCharacter|UseFocusConsumable)
      (Development|PrintString "Focus Used"))))

(event Input|ActionEvents|InputActionUse
  (params (Key :type Key%20Structure :default "None"))
  (:Pressed
    (if (== "/Script/VoidSpoken.HealthPickup" (Variables|VoidSpoken_GameMode_BP_C|GetCurrent%20Item (.AsVoid%20Spoken%20Game%20Mode%20BP (Utilities|Casting|CastToVoidSpoken_GameMode_BP (Game|GetGameMode)))))
      (Class|PlayerCharacter|UseHealthConsumable)
      (Development|PrintString "Health Used"))))

(fn ConstructionScript)