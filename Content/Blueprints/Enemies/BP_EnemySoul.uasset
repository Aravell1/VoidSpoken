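; BP_EnemySoul is a soul effect that flies from its spawn location to the crystal of its owning Obelisk and adds a charge to it.
; On BeginPlay it builds a three-point spline to the CrystalPos socket, with a raised quarter-way point bending the path.
; A timeline moves the actor along the spline, then deactivates the cloud, charges the Obelisk and destroys the actor after a short delay.
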(event Custom|UpdateSpline
  (bind _returnvalue (Transformation|GetActorLocation))
  (bind _asobelisk (Utilities|Casting|CastToObelisk (Components|GetOwner)))
  (Variables|Default|SetTargetObelisk _asobelisk)
  (Spline|SetSplinePoints (Variables|Default|GetSpline) (Utilities|Array|MakeArray _returnvalue (+ _returnvalue (+ (/ (- (Transformation|GetSocketLocation (Variables|/Script/VoidSpoken.Obelisk|GetObeliskMesh _asobelisk) "CrystalPos") _returnvalue) 4.0) (Math|Vector|MakeVector 0.0 0.0 (* (- (.z (Transformation|GetSocketLocation (Variables|/Script/VoidSpoken.Obelisk|GetObeliskMesh _asobelisk) "CrystalPos")) (.z (Transformation|GetActorLocation))) 0.35)))) (Transformation|GetSocketLocation (Variables|/Script/VoidSpoken.Obelisk|GetObeliskMesh _asobelisk) "CrystalPos")) "Local" true)
  (bind _time_track (Timeline|Position%20Timeline PlayFromStart)
    (:Update
      (Transformation|SetActorLocation (Spline|GetLocationatTime (Variables|Default|GetSpline) _time_track "Local" false) false false))
    (:Finished
      (Components|Activation|Deactivate (Variables|Default|GetCloud))
      (Class|Obelisk|AddCharge (Variables|Default|GetTargetObelisk))
      (Utilities|FlowControl|Delay 1.0)
      (Actor|DestroyActor))))

(event EventBeginPlay
  (CallFunction|UpdateSpline))

(event Collision|EventActorBeginOverlap
  (params (OtherActor :type Actor%20Object%20Reference)))

(event EventTick
  (params (DeltaSeconds :type Float%20%28single-precision%29)))

(fn ConstructionScript)