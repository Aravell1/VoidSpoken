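; Player character Blueprint that adds enemy lock-on targeting through a TargetingComponentTest component.
; BeginPlay initializes the component with the pawn, controller, mesh and a spine bone for the lock-on widget.
; Middle mouse triggers lock-on and TabTarget swaps targets, while mouse look axes pass through the component before driving controller yaw and pitch.
; TargetInformations exposes the component to callers.
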(event EventBeginPlay
  (bind _self self)
  (|CallParentFunction)
  (Default|Initialization (Variables|Default|GetTargetingComponent_Test) _self (Pawn|GetController _self) (Variables|Character|GetMesh) "spine_05"))

(event Input|ActionEvents|InputActionTabTarget
  (params (Key :type Key%20Structure :default "None"))
  (:Pressed
    (Default|SwapTarget (Variables|Default|GetTargetingComponent_Test))))

(event Input|AxisEvents|InputAxisTurn/Mouse
  (params (AxisValue :type Float%20%28single-precision%29))
  (Pawn|Input|AddControllerYawInput (Default|AxisTurn (Variables|Default|GetTargetingComponent_Test) AxisValue)))

(event Input|AxisEvents|InputAxisLookup/downMouse
  (params (AxisValue :type Float%20%28single-precision%29))
  (Pawn|Input|AddControllerPitchInput (Default|AxisLookUp (Variables|Default|GetTargetingComponent_Test) AxisValue)))

(event Input|MouseEvents|MiddleMouseButton
  (params (Key :type Key%20Structure :default "None"))
  (:Pressed
    (Default|Lockon (Variables|Default|GetTargetingComponent_Test))))

(fn ConstructionScript
  (|CallParentFunction))

(fn TargetInformations
  (return (Variables|Default|GetTargetingComponent_Test)))