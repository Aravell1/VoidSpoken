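; Base enemy character that roams, chases and melee-attacks the player, with a health bar and timed removal after death.
; A behaviour-mode state machine alternates random roaming with returns to the nearest patrol point.
; Pawn sensing or player damage starts a chase, dropped if movement fails with the target out of range.
; Attacks play random montages while turning toward the target, using a notify-driven sphere trace to apply randomised damage.
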(event OnSeePawn(PawnSensing)
  (params (Pawn :type Pawn%20Object%20Reference))
  ;[1 1 1] Chases the player if spotted
  (if (not (Variables|Default|GetDead?))
    (Variables|/Script/Engine.CharacterMovementComponent|SetMaxWalkSpeed (Variables|Character|GetCharacterMovement) (Variables|Default|GetChaseSpeed))
    (bind _asplayer_character (Utilities|Casting|CastToPlayerCharacter Pawn))
    (Variables|Default|SetAttackTarget _asplayer_character)
    (Rendering|SetVisibility (Variables|Default|GetHPWidgetComponent) true false)
    (Variables|Default|SetBehaviourMode "NewEnumerator2")
    (CallFunction|BehaviourUnit)))

(event Custom|BehaviourUnit
  (bind _charactermovement (Variables|Character|GetCharacterMovement))
  ;[1 1 1] Enemy Behaviour Modes
  (if (not (Variables|Default|GetDead?))
    (switch Utilities|FlowControl|Switch|SwitchonBehaviourModes (Variables|Default|GetBehaviourMode)
      (:NewEnumerator0
        (Variables|/Script/Engine.CharacterMovementComponent|SetMaxWalkSpeed (Variables|Character|GetCharacterMovement) (Variables|Default|GetWalkSpeed))
        (AI|AIMoveTo self (.RandomLocation (AI|Navigation|GetRandomReachablePointinRadius (Transformation|GetActorLocation) (Variables|Default|GetRoamRadius) 0 0)) 0 5.0 false
          (:then
            (CallFunction|UpdatePatrolPoint)
            (Utilities|FlowControl|Delay (Math|Random|RandomFloatinRange (Variables|Default|GetMinWait) (Variables|Default|GetMaxWait)))
            (if (Utilities|Enum|Equal(Enum) (Variables|Default|GetBehaviourMode) "NewEnumerator2")
              (CallFunction|ChasePlayer :!label _label)
              (else
                (Variables|Default|SetBehaviourMode "NewEnumerator1")
                (CallFunction|BehaviourUnit))))))
      (:NewEnumerator1
        (Variables|/Script/Engine.CharacterMovementComponent|SetMaxWalkSpeed (Variables|Character|GetCharacterMovement) (Variables|Default|GetWalkSpeed))
        (AI|AIMoveTo self "0, 0, 0" (Variables|Default|GetPatrolPointRef) 5.0 false
          (:OnSuccess
            (Utilities|FlowControl|Delay (Math|Random|RandomFloatinRange (Variables|Default|GetMinWait) (Variables|Default|GetMaxWait)))
            (if (Utilities|Enum|Equal(Enum) (Variables|Default|GetBehaviourMode) "NewEnumerator2")
              (goto _label)
              (else
                (Variables|Default|SetBehaviourMode "NewEnumerator0")
                (CallFunction|BehaviourUnit))))))
      (:NewEnumerator2
        (if (not (Variables|Default|GetDead?))
          (AI|AIMoveTo self "0, 0, 0" (Variables|Default|GetAttackTarget) (Variables|Default|GetAttackAcceptanceRadius) false
            (:OnSuccess
              (Utilities|FlowControl|DoOnce false
                (:Completed
                  (Variables|Default|SetAttackingPlayer? true)
                  (bind _notifyname (Animation|Montage|PlayMontage (Variables|Character|GetMesh) (Utilities|Select :Index (Math|Random|RandomInteger (Variables|Default|GetEnemyAttackAmount)) :Option%200 (Variables|Default|GetAttackMontage) :Option%201 (Variables|Default|GetAttack2Montage) :Option%202 (Variables|Default|GetAttack3Montage) :Option%203 (Variables|Default|GetAttack4Montage)))
                    (:then
                      (Components|Movement|StopMovementImmediately _charactermovement)
                      (Variables|/Script/Engine.CharacterMovementComponent|SetMaxWalkSpeed _charactermovement 0.0)
                      (CallFunction|TrackPlayer))
                    (:OnCompleted
                      (Utilities|FlowControl|Delay (Math|Random|RandomFloatinRange 0.1 0.3))
                      (Variables|Default|SetAttackingPlayer? false)
                      (if (not (Variables|Default|GetDead?))
                        (CallFunction|ReleaseAttack)
                        (Variables|/Script/Engine.CharacterMovementComponent|SetMaxWalkSpeed (Variables|Character|GetCharacterMovement) (Variables|Default|GetChaseSpeed))
                        (CallFunction|BehaviourUnit)))
                    (:OnNotifyBegin
                      (switch name _notifyname
                        (:AttackTrace
                          (CallFunction|AttackTrace))))))))
            (:OnFail
              (CallFunction|ChaseDistanceCheck))))))))

(event Custom|ChasePlayer
  (bind _charactermovement (Variables|Character|GetCharacterMovement))
  ;[1 1 1] Enemy Behaviour Modes
  (if (not (Variables|Default|GetDead?))
    (AI|AIMoveTo self "0, 0, 0" (Variables|Default|GetAttackTarget) (Variables|Default|GetAttackAcceptanceRadius) false
      (:OnSuccess
        (Utilities|FlowControl|DoOnce false
          (:Completed
            (Variables|Default|SetAttackingPlayer? true)
            (bind _notifyname (Animation|Montage|PlayMontage (Variables|Character|GetMesh) (Utilities|Select :Index (Math|Random|RandomInteger (Variables|Default|GetEnemyAttackAmount)) :Option%200 (Variables|Default|GetAttackMontage) :Option%201 (Variables|Default|GetAttack2Montage) :Option%202 (Variables|Default|GetAttack3Montage) :Option%203 (Variables|Default|GetAttack4Montage)))
              (:then
                (Components|Movement|StopMovementImmediately _charactermovement)
                (Variables|/Script/Engine.CharacterMovementComponent|SetMaxWalkSpeed _charactermovement 0.0)
                (CallFunction|TrackPlayer))
              (:OnCompleted
                (Utilities|FlowControl|Delay (Math|Random|RandomFloatinRange 0.1 0.3))
                (Variables|Default|SetAttackingPlayer? false)
                (if (not (Variables|Default|GetDead?))
                  (CallFunction|ReleaseAttack)
                  (Variables|/Script/Engine.CharacterMovementComponent|SetMaxWalkSpeed (Variables|Character|GetCharacterMovement) (Variables|Default|GetChaseSpeed))
                  (CallFunction|BehaviourUnit)))
              (:OnNotifyBegin
                (switch name _notifyname
                  (:AttackTrace
                    (CallFunction|AttackTrace))))))))
      (:OnFail
        (CallFunction|ChaseDistanceCheck)))))

(event Custom|ReleaseAttack
  (bind _charactermovement (Variables|Character|GetCharacterMovement))
  ;[1 1 1] Enemy Behaviour Modes
  (Utilities|FlowControl|DoOnce false) ; enters at Reset
)

(event Custom|TrackPlayer
  ;[1 1 1] Rotates toward the player while attacking
  (Variables|Default|GetAttackTarget
    (:then
      (if (Variables|Default|GetAttackingPlayer?)
        (Transformation|SetActorRotation (Math|Rotator|MakeRotator 0.0 0.0 (.yaw (Math|Rotator|FindLookatRotation (Transformation|GetActorLocation) (Transformation|GetActorLocation (Variables|Default|GetAttackTarget))))))
        (Utilities|FlowControl|Delay 0.01)
        (CallFunction|TrackPlayer)))
    (:else)))

(event Custom|ChaseDistanceCheck
  ;[1 1 1] Stops chasing if the player is out of range
  (if (not (Variables|Default|GetDead?))
    (if (> (Math|Vector|Distance(Vector) (Transformation|GetActorLocation) (Transformation|GetActorLocation (Variables|Default|GetAttackTarget))) 2.5e+03)
      (Rendering|SetVisibility (Variables|Default|GetHPWidgetComponent) false false)
      (Variables|Default|SetBehaviourMode "NewEnumerator0")
      (CallFunction|BehaviourUnit))))

(event Custom|DamageTest
  ;[1 1 1] Damage Test
  (Game|Damage|ApplyDamage self 5.0 0 (Game|GetPlayerCharacter 0)))

(event Custom|Enemy%20Death
  (bind _mesh (Variables|Character|GetMesh))
  (bind _capsulecomponent (Variables|Collision|GetCapsuleComponent))
  (bind _hpwidgetcomponent (Variables|Default|GetHPWidgetComponent))
  (bind _returnvalue (Components|SkeletalMesh|GetAnimInstance _mesh))
  ;[1 1 1] Enemy Death Actions
  (Utilities|IsValid _hpwidgetcomponent
    (:Is%20Valid
      (Rendering|SetVisibility _hpwidgetcomponent false false)
      (Utilities|FlowControl|DoOnce false
        (:Completed
          (Variables|Default|SetDead? true)
          (Components|Movement|StopMovementImmediately (Variables|Character|GetCharacterMovement))
          (if (Class|AnimInstance|IsAnyMontagePlaying _returnvalue)
            (Animation|Montage|MontageStop _returnvalue 0.0 (Animation|Montage|GetCurrentActiveMontage _returnvalue)))
          (Variables|/Script/Engine.CharacterMovementComponent|SetMaxWalkSpeed (Variables|Character|GetCharacterMovement) 0.0)
          (Variables|Default|SetAttackingPlayer? false)
          (Variables|Default|SetBehaviourMode "NewEnumerator3")
          (CallFunction|BehaviourUnit)
          (Collision|SetCollisionResponsetoChannel _capsulecomponent "ECC_Visibility" "ECR_Ignore")
          (Collision|SetCollisionResponsetoChannel _capsulecomponent "ECC_Pawn" "ECR_Ignore")
          (Utilities|FlowControl|Delay 1e+01)
          (Actor|DestroyActor))))))

(event EventBeginPlay
  ;[1 1 1] Start Behaviour Modes And Set Health Bar Percentage
  (CallFunction|BehaviourUnit)
  (bind _asenemy_health_bar_widget (Utilities|Casting|CastToEnemyHealthBarWidget (UserInterface|GetWidget (Variables|Default|GetHPWidgetComponent))))
  (bind _output_get (Variables|Default|SetEnemyHealthWidget _asenemy_health_bar_widget))
  (Default|UpdateHealth _output_get (/ (Math|Conversions|ToFloat(Integer) (Variables|Default|GetHealth)) (Math|Conversions|ToFloat(Integer) (Variables|Default|GetMaxHealth)))))

(event Game|Damage|EventAnyDamage
  (params (Damage :type Float%20%28single-precision%29) (DamageType :type Damage%20Type%20Object%20Reference) (InstigatedBy :type Controller%20Object%20Reference) (DamageCauser :type Actor%20Object%20Reference))
  (bind _returnvalue (Game|GetPlayerCharacter 0))
  ;[1 1 1] When The Enemy Takes Damage
  (if (== DamageCauser _returnvalue)
    (bind _asplayer_character (Utilities|Casting|CastToPlayerCharacter _returnvalue))
    (Variables|Default|SetAttackTarget _asplayer_character)
    (Variables|Default|SetBehaviourMode "NewEnumerator2")
    (CallFunction|ChasePlayer)
    (Variables|/Script/Engine.CharacterMovementComponent|SetMaxWalkSpeed (Variables|Character|GetCharacterMovement) (Variables|Default|GetChaseSpeed)))
  (if (not (Variables|Default|GetDead?))
    (bind _output_get (Variables|Default|SetHealth (Math|Float|Truncate (- (Variables|Default|GetHealth) Damage))))
    (if (<= _output_get 0)
      (CallFunction|EnemyDeath)
      (else
        (Default|UpdateHealth (Variables|Default|GetEnemyHealthWidget) (/ (Math|Conversions|ToFloat(Integer) (Variables|Default|GetHealth)) (Math|Conversions|ToFloat(Integer) (Variables|Default|GetMaxHealth))))))))

(fn ConstructionScript
  (bind _self self)
  (bind _outactors (Actor|GetAllActorsOfClass "/Game/Blueprints/Enemies/EnemyPatrolPoint_BP.EnemyPatrolPoint_BP_C"))
  (Variables|Default|SetPatrolPointRef (Utilities|Array|Get(acopy) _outactors))
  (for _array_element _outactors
    (if (< (Transformation|GetDistanceTo _array_element _self) (Transformation|GetDistanceTo (Variables|Default|GetPatrolPointRef) _self))
      (Variables|Default|SetPatrolPointRef _array_element))))

(fn UpdatePatrolPoint
  (bind _self self)
  (bind _outactors (Actor|GetAllActorsOfClass "/Game/Blueprints/Enemies/EnemyPatrolPoint_BP.EnemyPatrolPoint_BP_C"))
  (for _array_element _outactors
    (if (< (Transformation|GetDistanceTo _array_element _self) (Transformation|GetDistanceTo (Variables|Default|GetPatrolPointRef) _self))
      (Variables|Default|SetPatrolPointRef _array_element))))

(fn AttackTrace
  (bind _returnvalue (Transformation|GetActorLocation))
  (bind _attack_dmg (Variables|Default|GetAttack%20DMG))
  (bind (_outhit _returnvalue_2) (Collision|SphereTraceByChannel _returnvalue (+ _returnvalue (* (Transformation|GetActorForwardVector) (Variables|Default|GetAttackRange))) (Variables|Default|GetAttackRadius) "TraceTypeQuery3" false 0 "ForDuration"))
  (if _returnvalue_2
    (Game|Damage|ApplyDamage (.HitActor (Collision|BreakHitResult _outhit)) (Math|Conversions|ToFloat(Integer) (Math|Float|Round (Math|Random|RandomFloatinRange (Math|Conversions|ToFloat(Integer) (- _attack_dmg 2)) (Math|Conversions|ToFloat(Integer) (+ _attack_dmg 2))))) 0 0)))