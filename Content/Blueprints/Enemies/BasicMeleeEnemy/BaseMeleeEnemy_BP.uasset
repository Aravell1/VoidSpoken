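; Base melee enemy AI that roams, chases the player on sight and attacks in melee.
; A BehaviourMode switch alternates AI moves between random nearby points and the nearest patrol point, with random waits.
; PawnSensing switches to chasing; on arrival a DoOnce-gated attack montage halts movement, then resumes the chase when finished.
; A montage notify fires a sphere trace that applies slightly randomized damage to whatever it hits.
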(event OnSeePawn(PawnSensing)
  (params (Pawn :type Pawn%20Object%20Reference))
  (if (not (Variables|Default|GetDead?))
    (bind _asplayer_character_bp (Utilities|Casting|CastToPlayerCharacter_BP Pawn))
    (Variables|Default|SetAttackTarget _asplayer_character_bp)
    (Variables|Default|SetBehaviourMode "NewEnumerator2")
    (CallFunction|BehaviourUnitSystem)))

(event Custom|BehaviourUnitSystem
  (bind _charactermovement (Variables|Character|GetCharacterMovement))
  (if (not (Variables|Default|GetDead?))
    (switch Utilities|FlowControl|Switch|SwitchonBehaviourModes (Variables|Default|GetBehaviourMode)
      (:NewEnumerator0
        (AI|AIMoveTo self (.RandomLocation (AI|Navigation|GetRandomReachablePointinRadius (Transformation|GetActorLocation) (Variables|Default|GetRoamRaidius) 0 0)) 0 5.0 false
          (:OnSuccess
            (CallFunction|UpdatePatrolPoint)
            (Utilities|FlowControl|Delay (Math|Random|RandomFloatinRange (Variables|Default|GetMinWait) (Variables|Default|GetMaxWait)))
            (if (Utilities|Enum|Equal(Enum) (Variables|Default|GetBehaviourMode) "NewEnumerator2")
              (CallFunction|ChasePlayer)
              (else
                (Variables|Default|SetBehaviourMode "NewEnumerator1")
                (CallFunction|BehaviourUnitSystem))))))
      (:NewEnumerator1
        (AI|AIMoveTo self "0, 0, 0" (Variables|Default|GetPatrolPointReference) 5.0 false
          (:OnSuccess
            (Utilities|FlowControl|Delay (Math|Random|RandomFloatinRange (Variables|Default|GetMinWait) (Variables|Default|GetMaxWait)))
            (if (Utilities|Enum|Equal(Enum) (Variables|Default|GetBehaviourMode) "NewEnumerator2")
              (CallFunction|ChasePlayer)
              (else
                (Variables|Default|SetBehaviourMode "NewEnumerator0")
                (CallFunction|BehaviourUnitSystem))))))
      (:NewEnumerator2
        (if (not (Variables|Default|GetDead?))
          (AI|AIMoveTo self "0, 0, 0" (Variables|Default|GetAttackTarget) (Variables|Default|GetAttackAcceptanceRange) false
            (:OnSuccess
              (Utilities|FlowControl|DoOnce false
                (:Completed
                  (Variables|Default|SetAttackingPlayer false)
                  (bind _notifyname (Animation|Montage|PlayMontage (Variables|Character|GetMesh) (Variables|Default|GetAttackMontage))
                    (:then
                      (Components|Movement|StopMovementImmediately _charactermovement)
                      (Variables|/Script/Engine.CharacterMovementComponent|SetMaxWalkSpeed _charactermovement 0.0)
                      (CallFunction|TrackPlayer))
                    (:OnCompleted
                      (Utilities|FlowControl|Delay (Math|Random|RandomFloatinRange 0.1 0.3))
                      (Variables|Default|SetAttackingPlayer false)
                      (if (not (Variables|Default|GetDead?))
                        (CallFunction|ReleaseAttack)
                        (Variables|/Script/Engine.CharacterMovementComponent|SetMaxWalkSpeed (Variables|Character|GetCharacterMovement) 4.5e+02)
                        (CallFunction|BehaviourUnitSystem)))
                    (:OnNotifyBegin
                      (switch name _notifyname
                        (:AttackTrace
                          (CallFunction|AttackTrace))))))))))))))

(event Custom|ChasePlayer
  (bind _charactermovement (Variables|Character|GetCharacterMovement))
  (if (not (Variables|Default|GetDead?))
    (AI|AIMoveTo self "0, 0, 0" (Variables|Default|GetAttackTarget) (Variables|Default|GetAttackAcceptanceRange) false
      (:OnSuccess
        (Utilities|FlowControl|DoOnce false
          (:Completed
            (Variables|Default|SetAttackingPlayer false)
            (bind _notifyname (Animation|Montage|PlayMontage (Variables|Character|GetMesh) (Variables|Default|GetAttackMontage))
              (:then
                (Components|Movement|StopMovementImmediately _charactermovement)
                (Variables|/Script/Engine.CharacterMovementComponent|SetMaxWalkSpeed _charactermovement 0.0)
                (CallFunction|TrackPlayer))
              (:OnCompleted
                (Utilities|FlowControl|Delay (Math|Random|RandomFloatinRange 0.1 0.3))
                (Variables|Default|SetAttackingPlayer false)
                (if (not (Variables|Default|GetDead?))
                  (CallFunction|ReleaseAttack)
                  (Variables|/Script/Engine.CharacterMovementComponent|SetMaxWalkSpeed (Variables|Character|GetCharacterMovement) 4.5e+02)
                  (CallFunction|BehaviourUnitSystem)))
              (:OnNotifyBegin
                (switch name _notifyname
                  (:AttackTrace
                    (CallFunction|AttackTrace)))))))))))

(event Custom|ReleaseAttack
  (bind _charactermovement (Variables|Character|GetCharacterMovement))
  (Utilities|FlowControl|DoOnce false) ; enters at Reset
)

(event Custom|TrackPlayer
  (Variables|Default|GetAttackTarget
    (:then
      (if (Variables|Default|GetAttackingPlayer)
        (Transformation|SetActorRotation (Math|Rotator|FindLookatRotation (Transformation|GetActorLocation) (Transformation|GetActorLocation (Variables|Default|GetAttackTarget))))
        (Utilities|FlowControl|Delay 0.01)
        (CallFunction|TrackPlayer)))
    (:else)))

(event EventBeginPlay
  (CallFunction|BehaviourUnitSystem))

(event Collision|EventActorBeginOverlap
  (params (OtherActor :type Actor%20Object%20Reference)))

(event EventTick
  (params (DeltaSeconds :type Float%20%28single-precision%29)))

(fn ConstructionScript
  (bind _self self)
  (bind _outactors (Actor|GetAllActorsOfClass "/Game/Blueprints/Enemies/EnemyPatrolPoint_BP.EnemyPatrolPoint_BP_C"))
  (Variables|Default|SetPatrolPointReference (Utilities|Array|Get(acopy) _outactors))
  (for _array_element _outactors
    (if (< (Transformation|GetDistanceTo _array_element _self) (Transformation|GetDistanceTo _self (Variables|Default|GetPatrolPointReference)))
      (Variables|Default|SetPatrolPointReference _array_element))))

(fn UpdatePatrolPoint
  (bind _self self)
  (bind _outactors (Actor|GetAllActorsOfClass "/Game/Blueprints/Enemies/EnemyPatrolPoint_BP.EnemyPatrolPoint_BP_C"))
  (for _array_element _outactors
    (if (< (Transformation|GetDistanceTo _array_element _self) (Transformation|GetDistanceTo _self (Variables|Default|GetPatrolPointReference)))
      (Variables|Default|SetPatrolPointReference _array_element))))

(fn AttackTrace
  (bind _returnvalue (Transformation|GetActorLocation))
  (bind _attackdmg (Variables|Default|GetAttackDMG))
  (bind (_outhit _returnvalue_2) (Collision|SphereTraceByChannel _returnvalue (+ _returnvalue (+ (Transformation|GetActorForwardVector) (Variables|Default|GetAttackRange))) (Variables|Default|GetAttackRadius) "TraceTypeQuery1" false 0 "ForDuration"))
  (if _returnvalue_2
    (Game|Damage|ApplyDamage (.HitActor (Collision|BreakHitResult _outhit)) (Math|Conversions|ToFloat(Integer) (Math|Float|Round (Math|Random|RandomFloatinRange (- _attackdmg 2.0) (+ _attackdmg 2.0)))) 0 0)))