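; BP_PlayerSoul is a soul pickup actor that homes in on the player and triggers focus regeneration when it reaches them.
; Each tick it moves straight toward the cached player character at MoveSpeed, without sweep collision.
; Within MinRange it calls StartFocusRegen on the player, deactivates its Cloud effect, and destroys itself after a one-second delay.
; The range branch has no one-shot guard, so StartFocusRegen repeats each tick during that delay while the player stays in range.
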(event EventBeginPlay
  (bind _asplayer_character (Utilities|Casting|CastToPlayerCharacter (Game|GetPlayerCharacter 0)))
  (Variables|Default|SetPlayerRef _asplayer_character))

(event EventTick
  (params (DeltaSeconds :type Float%20%28single-precision%29))
  (bind _returnvalue (Transformation|GetActorLocation))
  (bind _playerref (Variables|Default|GetPlayerRef))
  (bind _returnvalue_2 (Transformation|GetActorLocation _playerref))
  (if (<= (Math|Vector|Distance(Vector) _returnvalue_2 _returnvalue) (Variables|Default|GetMinRange))
    (Class|PlayerCharacter|StartFocusRegen (Variables|Default|GetPlayerRef))
    (Components|Activation|Deactivate (Variables|Default|GetCloud))
    (Utilities|FlowControl|Delay 1.0)
    (Actor|DestroyActor)
    (else
      (Transformation|AddActorWorldOffset (* (* (Math|Vector|Normalize (- _returnvalue_2 _returnvalue)) (Variables|Default|GetMoveSpeed)) DeltaSeconds)))))

(fn ConstructionScript)