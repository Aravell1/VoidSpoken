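; Base Ghoul enemy Blueprint that drives an overhead health and stagger bar and exposes itself to the targeting system.
; BeginPlay caches the health bar widget, binds health updates and initializes the targeting component on a spine bone.
; Health updates reveal the bar and hide it at zero health.
; While the bar is visible, Tick rotates it toward the player camera and refreshes the stagger gauge when staggering is possible.
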(event Custom|UpdateHPBar
  (bind _stats (Variables|Default|GetStats))
  (bind _hpwidgetcomponent (Variables|Default|GetHPWidgetComponent))
  (bind _health (Variables|/Script/VoidSpoken.StatsMasterClass|GetHealth _stats))
  (if (Rendering|IsVisible _hpwidgetcomponent)
    _
    (else
      (Rendering|SetVisibility _hpwidgetcomponent true false)))
  (if (> _health 0.0)
    (Default|UpdateHealth (Variables|Default|GetHealthBar) (/ _health (Class|StatsMasterClass|GetMaxHealth _stats)))
    (else
      (Rendering|SetVisibility (Variables|Default|GetHPWidgetComponent) false false))))

(event EventBeginPlay
  (bind _self self)
  (bind _stats (Variables|Default|GetStats))
  (bind _asenemy_health_bar_widget (Utilities|Casting|CastToEnemyHealthBarWidget (UserInterface|GetWidget (Variables|Default|GetHPWidgetComponent))))
  (bind _output_get (Variables|Default|SetHealthBar _asenemy_health_bar_widget))
  (Default|UpdateHealth _output_get (/ (Variables|/Script/VoidSpoken.StatsMasterClass|GetHealth _stats) (Class|StatsMasterClass|GetMaxHealth _stats)))
  (EventDispatchers|AssignUpdateHealthBar (delegate Custom|UpdateHPBar))
  ;[0 0 0] Initialize Enemy Targeting
  (Default|Initialization (Variables|Default|GetTargetingComponent) _self (Pawn|GetController _self) (Variables|Character|GetMesh) "Spine2"))

(event EventTick
  (params (DeltaSeconds :type Float%20%28single-precision%29))
  (bind _staggercomponent (Variables|Default|GetStaggerComponent))
  (bind _hpwidgetcomponent (Variables|Default|GetHPWidgetComponent))
  (bind _staggerdamagethreshold (Variables|/Script/VoidSpoken.StaggerComponent|GetStaggerDamageThreshold _staggercomponent))
  (if (Rendering|IsVisible _hpwidgetcomponent)
    (Transformation|SetWorldRotation (Variables|Default|GetHPWidgetComponent) (Math|Rotator|FindLookatRotation (Transformation|GetWorldLocation _hpwidgetcomponent) (Camera|GetCameraLocation (Game|GetPlayerCameraManager 0))) false false)
    (if (Variables|/Script/VoidSpoken.StaggerComponent|GetbCanStagger (Variables|Default|GetStaggerComponent))
      (if (> _staggerdamagethreshold 0.0)
        (Default|UpdateStagger (Variables|Default|GetHealthBar) (/ (Class|StaggerComponent|GetStaggerGauge _staggercomponent) _staggerdamagethreshold))))))

(fn ConstructionScript)

(fn TargetDeadInformation
  (return (Variables|Default|GetbIsDead)))

(fn TargetInformations
  (return (Variables|Default|GetTargetingComponent)))