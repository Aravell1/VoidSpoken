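; Obelisk actor that charges as the player defeats enemies and shows its progress through a ring and a camera-facing charge bar widget.
; Enable, disable and update events drive ring and widget visibility and percentage.
; Disabling also reveals the active visual if activated, removes the compass tag and plays an Echo voiceline chosen by the CombatDirector's remaining obelisk count.
; Looking at it reports charge status; interaction always returns false.
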(event Custom|DisableCharge_Event
  (params (Obelisk :type Obelisk%20Object%20Reference))
  (if (Utilities|Enum|Equal(Enum) (Class|Obelisk|GetObeliskState) "Activated")
    (Rendering|SetVisibility (Variables|Default|GetObeliskActive) true false))
  (Rendering|SetVisibility (Variables|Default|GetRing) false false)
  (Widget|SetVisibility (Variables|Default|GetChargeBarWidget) "Hidden")
  (Utilities|Array|RemoveItem (Variables|Default|GetTags self) "Compass Interest")
  (CallFunction|PlayEchoVoiceline))

(event Custom|EnableCharge_Event
  (params (Obelisk :type Obelisk%20Object%20Reference))
  (CallFunction|SetRingHeight)
  (Rendering|SetVisibility (Variables|Default|GetRing) true false)
  (Widget|SetVisibility (Variables|Default|GetChargeBarWidget) "Visible")
  (Default|SetChargePercent (Variables|Default|GetChargeBarWidget)))

(event Custom|UpdateChargeWidget_Event
  (Default|SetChargePercent (Variables|Default|GetChargeBarWidget)))

(event EventBeginPlay
  (bind _asbp_obelisk_charge_widget (Utilities|Casting|CastToBP_ObeliskChargeWidget (UserInterface|GetWidget (Variables|Default|GetChargeBar))))
  (bind _output_get (Variables|Default|SetChargeBarWidget _asbp_obelisk_charge_widget))
  (Variables|/Game/Blueprints/Enviroment/Obelisk/BP_ObeliskChargeWidget.BP_ObeliskChargeWidget_C|SetObelisk _output_get self)
  (Widget|SetVisibility _output_get "Hidden")
  (EventDispatchers|AssignDisableCharge (delegate Custom|DisableCharge_Event))
  (EventDispatchers|AssignEnableCharge (delegate Custom|EnableCharge_Event))
  (EventDispatchers|AssignUpdateChargeWidget (delegate Custom|UpdateChargeWidget_Event)))

(event EventTick
  (params (DeltaSeconds :type Float%20%28single-precision%29))
  (CallFunction|SetChargeBarFacingCamera))

(fn ConstructionScript)

(fn SetRingHeight
  (bind _ring (Variables|Default|GetRing))
  (bind _ringthickness (Variables|Default|GetRingThickness))
  (Niagara|SetNiagaraVariable(Float) _ring "RingThickness" _ringthickness)
  (Transformation|AddRelativeLocation _ring (Math|Vector|MakeVector 0.0 0.0 (/ _ringthickness 2.0)) false false))

(fn SetChargeBarFacingCamera
  (bind _chargebar (Variables|Default|GetChargeBar))
  (if (Rendering|IsVisible _chargebar)
    (Transformation|SetWorldRotation (Variables|Default|GetChargeBar) (Math|Rotator|FindLookatRotation (Transformation|GetWorldLocation _chargebar) (Camera|GetCameraLocation (Game|GetPlayerCameraManager 0))) false false)))

(fn PlayEchoVoiceline
  (bind _returnvalue (Actor|GetActorOfClass "/Game/Blueprints/Enviroment/BP_PlayerPortal.BP_PlayerPortal_C"))
  (switch int (Class|CombatDirector|GetRemainingObeliskCount (Variables|/Game/Blueprints/Enviroment/BP_PlayerPortal.BP_PlayerPortal_C|GetCombatDirector _returnvalue))
    (:0
      (Audio|PlaySound2D "/Game/Assets/Audio/VOs/ECHO-WAV/ECHO-Line-N.ECHO-Line-N" 1.0 1.0 0.0 0 0))
    (:1
      (Audio|PlaySound2D "/Game/Assets/Audio/VOs/ECHO-WAV/ECHO-Line-M.ECHO-Line-M" 1.0 1.0 0.0 0 0))
    (:2
      (Audio|PlaySound2D "/Game/Assets/Audio/VOs/ECHO-WAV/ECHO-Line-L.ECHO-Line-L" 1.0 1.0 0.0 0 0))
    (:3
      (Audio|PlaySound2D "/Game/Assets/Audio/VOs/ECHO-WAV/ECHO-Line-K.ECHO-Line-K" 1.0 1.0 0.0 0 0))
    (:4
      (Audio|PlaySound2D "/Game/Assets/Audio/VOs/ECHO-WAV/ECHO-Line-J.ECHO-Line-J" 1.0 1.0 0.0 0 0))))

(fn Interactwith
  (params (Interactor :type Player%20Character%20BP%20Object%20Reference))
  (return false))

(fn LookatItem
  (params (Observer :type Player%20Character%20BP%20Object%20Reference))
  (bind _chargebarwidget (Variables|Default|GetChargeBarWidget))
  (bind _chargepercent (Variables|/Game/Blueprints/Enviroment/Obelisk/BP_ObeliskChargeWidget.BP_ObeliskChargeWidget_C|GetChargePercent _chargebarwidget))
  (Development|PrintString (Utilities|String|ToString(Float) _chargepercent))
  (if (>= _chargepercent 1.0)
    (return "Obelisk is fully charged!" "None")
    (else
      (return (Utilities|Text|ToText(String) (Utilities|String|Append "Defeat more enemies.Charged: " (Utilities|String|ToString(Float) (* _chargepercent 1e+02)) "%")) "None"))))