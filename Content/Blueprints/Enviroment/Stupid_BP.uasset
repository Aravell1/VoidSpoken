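; Stupid_BP is an environment actor that spins and bobs in place.
; It stores its starting Z on BeginPlay.
; Each Tick it adds a yaw rotation scaled by delta time and RotationRate, and sets its relative Z to that start plus a sine of time since creation, shaped by BobHeight and BobSpeed.
; The relative location is fed from world-space coordinates, so the two differ if the actor is attached to a parent.
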(event EventBeginPlay
  (Variables|Default|SetStartZ (.z (Transformation|GetActorLocation))))

(event Collision|EventActorBeginOverlap
  (params (OtherActor :type Actor%20Object%20Reference)))

(event EventTick
  (params (DeltaSeconds :type Float%20%28single-precision%29))
  (bind _returnvalue (Transformation|GetActorLocation))
  (Transformation|AddActorLocalRotation (Math|Rotator|MakeRotator 0.0 0.0 (* DeltaSeconds (Variables|Default|GetRotationRate))) false true)
  (Transformation|SetActorRelativeLocation (Math|Vector|MakeVector (.x _returnvalue) (.y _returnvalue) (+ (Variables|Default|GetStartZ) (* (Variables|Default|GetBobHeight) (Math|Trig|Sin(Radians) (* (Actor|GetGameTimeSinceCreation) (Variables|Default|GetBobSpeed))))))))

(fn ConstructionScript)