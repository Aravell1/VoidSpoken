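; BP_Obelisk is a world obelisk that shows its charge progress on a floating bar and reports it when looked at.
; On BeginPlay it links the bar widget to itself, hides it, and binds charge enable, disable and update events that control its visibility and percentage.
; Tick turns the visible bar toward the player camera.
; Looking returns a fully-charged or defeat-more-enemies message, while interaction always returns false.
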(event Custom|DisableCharge_Event
  (params (Obelisk :type Obelisk%20Object%20Reference))
  (Widget|SetVisibility (Variables|Default|GetChargeBarWidget) "Hidden"))

(event Custom|EnableCharge_Event
  (params (Obelisk :type Obelisk%20Object%20Reference))
  (Widget|SetVisibility (Variables|Default|GetChargeBarWidget) "Visible")
  (Default|SetChargePercent (Variables|Default|GetChargeBarWidget)))

(event Custom|UpdateChargeWidget_Event
  (Default|SetChargePercent (Variables|Default|GetChargeBarWidget)))

(event EventBeginPlay
  (bind _asbp_obelisk_charge_widget (Utilities|Casting|CastToBP_ObeliskChargeWidget (UserInterface|GetWidget (Variables|Default|GetChargeBar))))
  (bind _output_get (Variables|Default|SetChargeBarWidget _asbp_obelisk_charge_widget))
  (Variables|/Game/Blueprints/Enviroment/BP_ObeliskChargeWidget.BP_ObeliskChargeWidget_C|SetObelisk _output_get self)
  (Widget|SetVisibility _output_get "Hidden")
  (EventDispatchers|AssignDisableCharge (delegate Custom|DisableCharge_Event))
  (EventDispatchers|AssignEnableCharge (delegate Custom|EnableCharge_Event))
  (EventDispatchers|AssignUpdateChargeWidget (delegate Custom|UpdateChargeWidget_Event)))

(event EventTick
  (params (DeltaSeconds :type Float%20%28single-precision%29))
  (bind _chargebar (Variables|Default|GetChargeBar))
  (if (Rendering|IsVisible _chargebar)
    (Transformation|SetWorldRotation (Variables|Default|GetChargeBar) (Math|Rotator|FindLookatRotation (Transformation|GetWorldLocation _chargebar) (Camera|GetCameraLocation (Game|GetPlayerCameraManager 0))) false false)))

(fn ConstructionScript)

(fn Interactwith
  (params (Interactor :type Player%20Character%20BP%20Object%20Reference))
  (return false))

(fn LookatItem
  (params (Observer :type Player%20Character%20BP%20Object%20Reference))
  (bind _chargebarwidget (Variables|Default|GetChargeBarWidget))
  (bind _chargepercent (Variables|/Game/Blueprints/Enviroment/BP_ObeliskChargeWidget.BP_ObeliskChargeWidget_C|GetChargePercent _chargebarwidget))
  (Development|PrintString (Utilities|String|ToString(Float) _chargepercent))
  (if (>= _chargepercent 1.0)
    (return "Obelisk is fully charged!" "None")
    (else
      (return (Utilities|Text|ToText(String) (Utilities|String|Append "Defeat more enemies.Charged: " (Utilities|String|ToString(Float) (* _chargepercent 1e+02)) "%")) "None"))))