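; Portal actor that teleports the player to a linked TargetPortal, offset along its forward vector, matching its yaw and resetting the camera.
; Overlap by the player or their equipped weapon triggers travel only when the GameMode's obelisk count is zero or less and the CombatDirector found at BeginPlay reports no combat.
; InteractWith returns false; LookAtItem clears CanTravel before checking it, so it always shows the "finish combat" message.
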(event EventBeginPlay
  (bind _outactors (Actor|GetAllActorsOfClass "/Script/VoidSpoken.CombatDirector"))
  (for _array_element _outactors
    (Variables|Default|SetCombatDirector _array_element)))

(event Collision|EventActorBeginOverlap
  (params (OtherActor :type Actor%20Object%20Reference))
  (bind _returnvalue (Game|GetPlayerCharacter 0))
  (bind _targetportal (Variables|Default|GetTargetPortal))
  (bind _combatdirector (Variables|Default|GetCombatDirector))
  (bind _asplayer_character_bp (Utilities|Casting|CastToPlayerCharacter_BP _returnvalue))
  (bind _asvoid_spoken_game_mode_bp (Utilities|Casting|CastToVoidSpoken_GameMode_BP (Game|GetGameMode)))
  (if (<= (Class|VoidSpokenGameModeBase|GetObeliskCount _asvoid_spoken_game_mode_bp) 0)
    (Utilities|IsValid _combatdirector
      (:Is%20Valid
        (bind _returnvalue_2 (Class|CombatDirector|GetinCombat _combatdirector))
        (if (not _returnvalue_2)
          (Utilities|Casting|CastToPlayerCharacter_BP OtherActor
            (:then
              (Utilities|IsValid _targetportal :!label _label
                (:Is%20Valid
                  (Variables|Default|SetCanTravel true)
                  (Development|PrintString "You can travel through!" true true "(R=0.000000,G=0.660000,B=1.000000,A=1.000000)" 3.0)
                  (Transformation|Teleport _asplayer_character_bp (+ (Transformation|GetActorLocation _targetportal) (* (Transformation|GetActorForwardVector _targetportal) (Variables|Default|GetSpawnDistance))) (Math|Rotator|MakeRotator 0.0 0.0 (.yaw (Transformation|GetActorRotation _targetportal))))
                  (Class|PlayerCharacter|ResetCameraRotation _asplayer_character_bp))
                (:Is%20Not%20Valid
                  (Variables|Default|SetCanTravel true)
                  (Development|PrintString "You can't travel through. Finish combat." true true "(R=0.000000,G=0.660000,B=1.000000,A=1.000000)" 5.0))))
            (:CastFailed
              (if (== OtherActor (Variables|/Script/VoidSpoken.PlayerCharacter|GetEquippedWeapon _asplayer_character_bp))
                (goto _label)))))))))

(fn ConstructionScript)

(fn Interactwith
  (params (Interactor :type Player%20Character%20BP%20Object%20Reference))
  (return false))

(fn LookatItem
  (params (Observer :type Player%20Character%20BP%20Object%20Reference))
  (bind _output_get (Variables|Default|SetCanTravel false))
  (if _output_get
    (return "You can travel through. Be ready!" "None")
    (else
      (return "You can't travel through. Finish combat." "None"))))