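; Gatekeeper boss portal actor that spawns a single enemy, then removes itself.
; After a short delay on BeginPlay, it randomly selects a knight or ghoul class using EnemyCount and spawns it near the portal with yaw toward the player.
; It then casts the spawn to BaseEnemy_BP and calls SeePlayer with the player character to alert it.
; If both casts succeed, the portal destroys itself after a further delay.
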(event EventBeginPlay
  (bind _returnvalue (Transformation|GetActorLocation))
  (bind _returnvalue_2 (Transformation|GetActorRotation))
  (bind _returnvalue_3 (Math|Random|RandomFloatinRange -5e+01 5e+01))
  (Utilities|FlowControl|Delay 1.5)
  (bind _returnvalue_4 (Game|SpawnActorfromClass (Utilities|Select :Index (Math|Random|RandomInteger (Variables|Default|GetEnemyCount)) :Option%200 "/Game/Blueprints/Enemies/KnightEnemy/KnightEnemy_BP.KnightEnemy_BP_C" :Option%201 "/Game/Blueprints/Enemies/BasicMeleeEnemy/Ghoul_BP.Ghoul_BP_C") (Math|Transform|MakeTransform (Math|Vector|MakeVector (+ (.x _returnvalue) _returnvalue_3) (+ (.y _returnvalue) _returnvalue_3) 0.0) (Math|Rotator|MakeRotator (.roll _returnvalue_2) (.pitch _returnvalue_2) (.yaw (Math|Rotator|FindLookatRotation (Transformation|GetActorLocation) (Transformation|GetActorLocation (Game|Player|GetPlayerPawn 0))))) (Transformation|GetActorScale3D)) "Undefined" 0 0))
  (Utilities|FlowControl|Delay 0.2)
  (bind _asbase_enemy_bp (Utilities|Casting|CastToBaseEnemy_BP _returnvalue_4))
  (bind _asplayer_character (Utilities|Casting|CastToPlayerCharacter (Game|GetPlayerCharacter 0)))
  (Default|SeePlayer _asbase_enemy_bp _asplayer_character)
  (Utilities|FlowControl|Delay 6.5)
  (Actor|DestroyActor))

(fn ConstructionScript)