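; Gatekeeper boss character that starts chasing and attacking the player once pawn sensing spots them.
; A state-driven BehaviourState event alternates a base attack with a random heavy attack, gated by resettable do-once nodes, while a recursive delayed lerp slowly turns it toward its target.
; Defense-scaled damage updates the health widget and, at each quarter-health threshold, summons progressively more portals, with the last triggering a faster, stronger enrage.
; The Death event is empty.
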(event OnSeePawn(PawnSensing)
  (params (Pawn :type Pawn%20Object%20Reference))
  ;[1 1 1] On See Player begin main action loop
  (Utilities|FlowControl|DoOnce false
    (:Completed
      (bind _asplayer_character_bp (Utilities|Casting|CastToPlayerCharacter_BP Pawn))
      (Variables|Default|SetattackTarget _asplayer_character_bp)
      (Variables|/Script/Engine.CharacterMovementComponent|SetMaxWalkSpeed (Variables|Character|GetCharacterMovement) (Variables|Default|GetwalkSpeed))
      (Rendering|SetVisibility (Variables|Default|GetHPWidgetComponent) true false)
      (Variables|Default|SetState "NewEnumerator0")
      (CallFunction|BehaviourState))))

(event Custom|BehaviourState
  (bind _charactermovement (Variables|Character|GetCharacterMovement))
  (bind _charactermovement_2 (Variables|Character|GetCharacterMovement))
  (bind _charactermovement_3 (Variables|Character|GetCharacterMovement))
  (bind _charactermovement_4 (Variables|Character|GetCharacterMovement))
  (bind _charactermovement_5 (Variables|Character|GetCharacterMovement))
  ;[1 1 1] Main Action Loop
  (switch Utilities|FlowControl|Switch|SwitchonGatekeeperStates (Variables|Default|GetState)
    (:NewEnumerator3
      (AI|AIMoveTo self "0, 0, 0" (Variables|Default|GetStartLocation) 5.0 false))
    (:NewEnumerator0
      (AI|AIMoveTo self "0, 0, 0" (Variables|Default|GetattackTarget) 4e+02 false
        (:OnSuccess
          (Utilities|FlowControl|DoOnce false
            (:Completed
              (Animation|Montage|PlayMontage (Variables|Character|GetMesh) (Variables|Default|GetBaseAttackMontage)
                (:then
                  (Components|Movement|StopMovementImmediately _charactermovement_3)
                  (Variables|/Script/Engine.CharacterMovementComponent|SetMaxWalkSpeed _charactermovement_3 0.0)
                  (Variables|Default|Setattacking true)
                  (CallFunction|TrackPlayer))
                (:OnCompleted
                  (Variables|Default|Setattacking false)
                  (if (Variables|Default|Getenraged)
                    (Variables|/Script/Engine.CharacterMovementComponent|SetMaxWalkSpeed _charactermovement_4 (Variables|Default|GetrunSpeed))
                    (else
                      (Variables|/Script/Engine.CharacterMovementComponent|SetMaxWalkSpeed _charactermovement_4 (Variables|Default|GetwalkSpeed))))
                  (CallFunction|ReleaseAttack)
                  (Variables|Default|SetState "NewEnumerator4")
                  (CallFunction|BehaviourState))))))))
    (:NewEnumerator4
      (AI|AIMoveTo self "0, 0, 0" (Variables|Default|GetattackTarget) 4e+02 false
        (:OnSuccess
          (Utilities|FlowControl|DoOnce false
            (:Completed
              (Animation|Montage|PlayMontage (Variables|Character|GetMesh) (Utilities|Select :Index (Math|Random|RandomInteger 2) :Option%200 (Variables|Default|GetHeavySwingMontage) :Option%201 (Variables|Default|GetStompMontage) :Option%202 (Variables|Default|GetBeamMontage))
                (:then
                  (Components|Movement|StopMovementImmediately _charactermovement_5)
                  (Variables|/Script/Engine.CharacterMovementComponent|SetMaxWalkSpeed _charactermovement_5 0.0)
                  (Variables|Default|Setattacking true)
                  (CallFunction|TrackPlayer))
                (:OnCompleted
                  (Variables|Default|Setattacking false)
                  (CallFunction|ReleaseHeavy)
                  (Utilities|FlowControl|Delay (Math|Random|RandomFloatinRange 2.5 3.5))
                  (if (Variables|Default|Getenraged)
                    (Variables|/Script/Engine.CharacterMovementComponent|SetMaxWalkSpeed _charactermovement (Variables|Default|GetrunSpeed))
                    (else
                      (Variables|/Script/Engine.CharacterMovementComponent|SetMaxWalkSpeed _charactermovement (Variables|Default|GetwalkSpeed))))
                  (Variables|Default|SetState "NewEnumerator0")
                  (CallFunction|BehaviourState))))))))
    (:NewEnumerator1
      (Variables|Default|Setattacking false)
      (Utilities|FlowControl|DoOnce false
        (:Completed
          (Animation|Montage|PlayMontage (Variables|Character|GetMesh) (Variables|Default|GetPortalMontage) 0.4
            (:then
              (Components|Movement|StopMovementImmediately _charactermovement_2)
              (Variables|/Script/Engine.CharacterMovementComponent|SetMaxWalkSpeed _charactermovement_2 0.0))
            (:OnCompleted
              (Utilities|FlowControl|Delay 1.0)
              (if (<= (Variables|Default|Gethealth) (* (Variables|Default|GetmaxHealth) 0.25))
                (CallFunction|ReleaseAttack)
                (CallFunction|ReleaseHeavy)
                (CallFunction|Enrage)
                (else
                  (CallFunction|PortalReset)
                  (Variables|/Script/Engine.CharacterMovementComponent|SetMaxWalkSpeed (Variables|Character|GetCharacterMovement) (Variables|Default|GetwalkSpeed))
                  (CallFunction|ReleaseAttack)
                  (CallFunction|ReleaseHeavy)
                  (Variables|Default|SetState "NewEnumerator0")
                  (CallFunction|BehaviourState))))))))))

(event Custom|TrackPlayer
  ;[1 1 1] Follow player slowly while attacking
  (Transformation|SetActorRotation (Math|Rotator|Lerp(Rotator) (Math|Rotator|MakeRotator 0.0 0.0 (.yaw (Transformation|GetActorRotation))) (Math|Rotator|MakeRotator 0.0 0.0 (.yaw (Math|Rotator|FindLookatRotation (Transformation|GetActorLocation) (Transformation|GetActorLocation (Variables|Default|GetAttackTarget))))) 0.02 true))
  (Utilities|FlowControl|Delay 0.01)
  (if (Variables|Default|Getattacking)
    (CallFunction|TrackPlayer)))

(event Custom|Enrage
  ;[1 1 1] Enrage
  (Variables|Default|Setenraged true)
  (Variables|Default|Setattack (* (Variables|Default|Getattack) 1.25))
  (Animation|Montage|PlayMontage (Variables|Character|GetMesh) (Variables|Default|GetEnrageMontage) 0.5
    (:OnCompleted
      (Variables|/Script/Engine.CharacterMovementComponent|SetMaxWalkSpeed (Variables|Character|GetCharacterMovement) (Variables|Default|GetrunSpeed))
      (Variables|Default|SetState "NewEnumerator0")
      (CallFunction|BehaviourState))))

(event Custom|ReleaseAttack
  (bind _charactermovement (Variables|Character|GetCharacterMovement))
  (bind _charactermovement_2 (Variables|Character|GetCharacterMovement))
  ;[1 1 1] Main Action Loop
  (Utilities|FlowControl|DoOnce false) ; enters at Reset
)

(event Custom|Death
  ;[1 1 1] Death
)

(event Custom|ReleaseHeavy
  (bind _charactermovement (Variables|Character|GetCharacterMovement))
  (bind _charactermovement_2 (Variables|Character|GetCharacterMovement))
  ;[1 1 1] Main Action Loop
  (Utilities|FlowControl|DoOnce false) ; enters at Reset
)

(event Custom|Portal%20Reset
  (bind _charactermovement (Variables|Character|GetCharacterMovement))
  ;[1 1 1] Main Action Loop
  (Utilities|FlowControl|DoOnce false) ; enters at Reset
)

(event EventBeginPlay
  ;[1 1 1] Begin Play
  (|CallParentFunction)
  (Variables|Default|SetState "NewEnumerator3")
  (CallFunction|BehaviourState))

(event Game|Damage|EventAnyDamage
  (params (Damage :type Float%20%28single-precision%29) (DamageType :type Damage%20Type%20Object%20Reference) (InstigatedBy :type Controller%20Object%20Reference) (DamageCauser :type Actor%20Object%20Reference))
  ;[1 1 1] On Damage Taken
  (Variables|Default|SetDamage (/ (* Damage 1e+01) (Variables|Default|Getdefense)))
  (if (and (> (Variables|Default|Gethealth) (* (Variables|Default|GetmaxHealth) 0.75)) (<= (- (Variables|Default|Gethealth) (Variables|Default|GetDamage)) (* (Variables|Default|GetmaxHealth) 0.75)))
    (Variables|Default|Sethealth (- (Variables|Default|Gethealth) (Variables|Default|GetDamage)))
    (Variables|/Script/Engine.CharacterMovementComponent|SetMaxWalkSpeed (Variables|Character|GetCharacterMovement) 0.0)
    (Default|UpdateHealth (Variables|Default|GetBossHealthWidget) (/ (Variables|Default|Gethealth) (Variables|Default|GetmaxHealth)))
    (CallFunction|SummonPortals 1)
    (Variables|Default|SetState "NewEnumerator1")
    (CallFunction|BehaviourState)
    (elif (and (> (Variables|Default|Gethealth) (* (Variables|Default|GetmaxHealth) 0.5)) (<= (- (Variables|Default|Gethealth) (Variables|Default|GetDamage)) (* (Variables|Default|GetmaxHealth) 0.5)))
      (Variables|Default|Sethealth (- (Variables|Default|Gethealth) (Variables|Default|GetDamage)))
      (Variables|/Script/Engine.CharacterMovementComponent|SetMaxWalkSpeed (Variables|Character|GetCharacterMovement) 0.0)
      (Default|UpdateHealth (Variables|Default|GetBossHealthWidget) (/ (Variables|Default|Gethealth) (Variables|Default|GetmaxHealth)))
      (CallFunction|SummonPortals 2)
      (Variables|Default|SetState "NewEnumerator1")
      (CallFunction|BehaviourState)
      (elif (and (> (Variables|Default|Gethealth) (* (Variables|Default|GetmaxHealth) 0.25)) (<= (- (Variables|Default|Gethealth) (Variables|Default|GetDamage)) (* (Variables|Default|GetmaxHealth) 0.25)))
        (Variables|Default|Sethealth (- (Variables|Default|Gethealth) (Variables|Default|GetDamage)))
        (Variables|/Script/Engine.CharacterMovementComponent|SetMaxWalkSpeed (Variables|Character|GetCharacterMovement) 0.0)
        (Default|UpdateHealth (Variables|Default|GetBossHealthWidget) (/ (Variables|Default|Gethealth) (Variables|Default|GetmaxHealth)))
        (CallFunction|SummonPortals 3)
        (Variables|Default|SetState "NewEnumerator1")
        (CallFunction|BehaviourState)
        (else
          (Variables|Default|Sethealth (- (Variables|Default|Gethealth) (Variables|Default|GetDamage)))
          (Default|UpdateHealth (Variables|Default|GetBossHealthWidget) (/ (Variables|Default|Gethealth) (Variables|Default|GetmaxHealth)))
          (if (<= (Variables|Default|Gethealth) 0.0)
            (CallFunction|Death)))))))

(fn ConstructionScript
  (|CallParentFunction))

(fn SummonPortals
  (params (portalCount :type Integer))
  (LocalVariables|Setcount portalCount)
  (Game|SpawnActorfromClass "/Game/Assets/Portal_BP.Portal_BP_C" (Transformation|GetActorTransform (Variables|Default|GetportalSpawnLeft)) "Undefined" 0 0)
  (if (>= (LocalVariables|Getcount) 2)
    (Game|SpawnActorfromClass "/Game/Assets/Portal_BP.Portal_BP_C" (Transformation|GetActorTransform (Variables|Default|GetportalSpawnRight)) "Undefined" 0 0)
    (if (>= (LocalVariables|Getcount) 3)
      (Game|SpawnActorfromClass "/Game/Assets/Portal_BP.Portal_BP_C" (Transformation|GetActorTransform (Variables|Default|GetportalSpawnForward)) "Undefined" 0 0))))