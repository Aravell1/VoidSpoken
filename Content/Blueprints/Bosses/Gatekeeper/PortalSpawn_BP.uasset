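; PortalSpawn_BP is a Gatekeeper boss Blueprint that handles enemies spawned for the fight.
; OrderAttack walks the game mode's GatekeeperEnemySpawns list, disables each enemy's reset and makes it see the player unless already targeting them.
; DisableEnemyHealthBar hides the HP widget on spawned ghouls.
; The file contains no spawn logic, and its OrderAttack delegate binding is left unconnected.
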(event Custom|OrderAttack
  (bind _returnvalue (Game|GetPlayerCharacter 0))
  (bind _asvoid_spoken_game_mode_bp (Utilities|Casting|CastToVoidSpoken_GameMode_BP (Game|GetGameMode)))
  (for _array_element (Variables|/Script/VoidSpoken.VoidSpokenGameModeBase|GetGatekeeperEnemySpawns _asvoid_spoken_game_mode_bp)
    (bind _asbase_enemy_bp (Utilities|Casting|CastToBaseEnemy_BP _array_element))
    (Variables|/Game/Blueprints/Enemies/BaseEnemy_BP.BaseEnemy_BP_C|SetCanReset _asbase_enemy_bp false)
    (if (not (== (Variables|/Game/Blueprints/Enemies/BaseEnemy_BP.BaseEnemy_BP_C|GetAttackTarget _asbase_enemy_bp) _returnvalue))
      (Default|SeePlayer _asbase_enemy_bp _returnvalue))))

(event EventBeginPlay)

(event EventDisableEnemyHealthBar
  (params (SpawnedEnemy :type Base%20Enemy%20Object%20Reference))
  (bind _asbp_base_ghoul (Utilities|Casting|CastToBP_Base_Ghoul SpawnedEnemy))
  (Development|SetHiddeninGame (Variables|/Game/Blueprints/Enemies/Ghoul/BP_Base_Ghoul.BP_Base_Ghoul_C|GetHPWidgetComponent _asbp_base_ghoul) true false))

(fn ConstructionScript)