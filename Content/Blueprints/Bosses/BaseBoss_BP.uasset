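; Base boss Blueprint that shows the boss's health on an enemy health bar widget.
; On BeginPlay it casts its widget component's widget to EnemyHealthBarWidget, caches it and initializes it with the current-to-max health ratio.
; A DamageTest event applies a tenth of max health as damage to the boss itself.
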(event Custom|DamageTest
  (Game|Damage|ApplyDamage self (/ (Variables|Default|GetMaxHealth) 1e+01) 0 0))

(event EventBeginPlay
  (bind _asenemy_health_bar_widget (Utilities|Casting|CastToEnemyHealthBarWidget (UserInterface|GetWidget (Variables|Default|GetHPWidgetComponent))))
  (bind _output_get (Variables|Default|SetBossHealthWidget _asenemy_health_bar_widget))
  (Default|UpdateHealth _output_get (/ (Variables|Default|GetHealth) (Variables|Default|GetMaxHealth))))

(event Collision|EventActorBeginOverlap
  (params (OtherActor :type Actor%20Object%20Reference)))

(event EventTick
  (params (DeltaSeconds :type Float%20%28single-precision%29)))

(fn ConstructionScript)