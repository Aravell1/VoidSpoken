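; Weapon Blueprint for the Gatekeeper that equips itself when play begins.
; BeginPlay loops over every Gatekeeper actor, calls Equip, sets itself as that actor's EquippedWeapon and attaches to the equipped character mesh's WeaponSocket if it exists.
; The same weapon instance is assigned to each Gatekeeper found.
; The logic is marked to switch to C++.
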(event EventBeginPlay
  (bind _equippedcharacter (Variables|Default|GetEquippedCharacter))
  (bind _mesh (Variables|/Script/Engine.Character|GetMesh _equippedcharacter))
  ;[1 1 1] Switch to C++
  (bind _outactors (Actor|GetAllActorsOfClass "/Script/VoidSpoken.Gatekeeper"))
  (for _array_element _outactors
    (Class|BaseWeapon|Equip self _array_element)
    (bind _output_get (Variables|/Script/VoidSpoken.PlayerCharacter|SetEquippedWeapon _array_element self))
    (if (Transformation|DoesSocketExist _mesh "WeaponSocket")
      (Transformation|AttachComponentToComponent _output_get _mesh "WeaponSocket" "KeepRelative" "KeepRelative" "KeepRelative" false))))

(event Collision|EventActorBeginOverlap
  (params (OtherActor :type Actor%20Object%20Reference)))

(event EventTick
  (params (DeltaSeconds :type Float%20%28single-precision%29)))

(fn ConstructionScript)