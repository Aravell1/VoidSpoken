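; Test weapon Blueprint that equips itself to the first player character when play begins.
; BeginPlay calls Equip on that character, then casts it to BaseEntity and registers itself as the EquippedWeapon.
; If the equipped character's mesh has a "Weapon Point" socket, it snaps onto that socket.
; A note marks this logic to be switched to C++.
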(event EventBeginPlay
  (bind _returnvalue (Game|GetPlayerCharacter 0))
  (bind _equippedcharacter (Variables|Default|GetEquippedCharacter))
  (bind _mesh (Variables|/Script/Engine.Character|GetMesh _equippedcharacter))
  ;[1 1 1] Switch to C++
  (Class|BaseWeapon|Equip self _returnvalue)
  (bind _asbase_entity (Utilities|Casting|CastToBaseEntity _returnvalue))
  (Variables|/Script/VoidSpoken.BaseEntity|SetEquippedWeapon _asbase_entity self)
  (if (Transformation|DoesSocketExist _mesh "Weapon Point")
    (Transformation|AttachComponentToComponent _mesh "Weapon Point" "SnapToTarget" "SnapToTarget" "SnapToTarget" false)))

(fn ConstructionScript)