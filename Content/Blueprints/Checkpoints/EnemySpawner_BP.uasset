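; Checkpoint enemy spawner that spawns a set number of Ghoul_BP AI pawns once at BeginPlay, after a short delay.
; Each ghoul lands at a random point in a box centered on the Arrow component, using the SpawnArea extent that the construction script sets from SpawnExtent.
; IsAlreadySpawned guards against repeat activation.
; The distance-check timer is unfinished: its setup never runs and its event does nothing.
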(event Custom|Spawn%20Timer
  (if (<= (Transformation|GetDistanceTo (Game|GetPlayerCharacter 0) 0) 0.0)
    _))

(event EventBeginPlay
  (CallFunction|ActivateEnemySpawner)
  (Variables|Default|SetbIsAlreadySpawned true))

(event EventActivateEnemySpawner
  (if (not (Variables|Default|GetbIsAlreadySpawned))
    (Utilities|FlowControl|Delay 1.0)
    (for _index (range 0 (- (Variables|Default|GetNumOfSpawn) 1))
      (AI|SpawnAIFromClass "/Game/Blueprints/Enemies/BasicMeleeEnemy/Ghoul_BP.Ghoul_BP_C" 0 (Math|Random|RandomPointinBoundingBox (Transformation|GetWorldLocation (Variables|Default|GetArrow)) (Variables|/Script/Engine.BoxComponent|GetBoxExtent (Variables|Default|GetSpawnArea))) "0, 0, 0" false 0)
      (Development|PrintString "Spawned"))
    (else
      (Development|PrintString "Already Spawned"))))

(fn ConstructionScript
  (Components|Box|SetBoxExtent (Variables|Default|GetSpawnArea) (Variables|Default|GetSpawnExtent) true))