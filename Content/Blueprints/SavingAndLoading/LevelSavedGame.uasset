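; LevelSavedGame is a save game object that stores and restores the inventory contents of a level's containers.
; SaveContainerInfo appends a container reference and its InventoryComponent contents to the Containers array, then writes itself to its save slot and prints a confirmation.
; LoadContainerInfo copies saved contents back into the matching container and removes that entry during the loop, without re-saving to the slot.
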(fn SaveContainerInfo
  (params (Container :type Actor%20Object%20Reference))
  (bind _returnvalue (Actor|GetComponentbyClass Container "/Game/Blueprints/SavingAndLoading/InventorySaving/InventoryComponent.InventoryComponent_C"))
  (bind _slot_name (Variables|Default|GetSlot%20Name))
  (Utilities|IsValid _returnvalue
    (:Is%20Valid
      (Utilities|Array|Add (Variables|Default|GetContainers) (Utilities|Struct|MakeContainerContentStruct (Utilities|ResolveSoftReference Container) (Variables|/Game/Blueprints/SavingAndLoading/InventorySaving/InventoryComponent.InventoryComponent_C|GetInventoryContent _returnvalue)))
      (SaveGame|SaveGametoSlot self _slot_name)
      (Development|PrintString 0 (Utilities|String|Append "Container has been saved to: " _slot_name)))))

(fn LoadContainerInfo
  (params (Container :type Actor%20Object%20Reference))
  (for (_array_element _array_index) (Variables|Default|GetContainers)
    (Variables|Default|SetCurrentIndex _array_index)
    (if (== (Utilities|ResolveSoftReference (.Container (Utilities|Struct|BreakContainerContentStruct _array_element))) Container)
      (Variables|/Game/Blueprints/SavingAndLoading/InventorySaving/InventoryComponent.InventoryComponent_C|SetInventoryContent (Actor|GetComponentbyClass Container "/Game/Blueprints/SavingAndLoading/InventorySaving/InventoryComponent.InventoryComponent_C") (.InventoryContent (Utilities|Struct|BreakContainerContentStruct _array_element)))
      (Utilities|Array|RemoveIndex (Variables|Default|GetContainers) (Variables|Default|GetCurrentIndex)))))