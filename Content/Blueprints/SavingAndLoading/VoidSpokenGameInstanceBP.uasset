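; Game Instance for Void Spoken that owns saving and loading of player and inventory data.
; On Init it loads or creates separate master, inventory and level save objects, though level data is only initialized here.
; Player functions copy health, stamina, focus and transform, writing the slot after each field on save but restoring only location from the transform.
; Inventory functions copy the inventory component's contents, with debug prints throughout.
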(event EventInit
  (bind _savedgamename (Variables|Default|GetSavedGameName))
  (bind _inventorysavegamename (Variables|Default|GetInventorySaveGameName))
  (bind _levelsavegamename (Variables|Default|GetLevelSaveGameName))
  (Utilities|FlowControl|Sequence
    (:then_0
      (bind _returnvalue (SaveGame|DoesSaveGameExist _savedgamename))
      (if (not _returnvalue)
        (bind _returnvalue_2 (SaveGame|CreateSaveGameObject "/Game/Blueprints/SavingAndLoading/MasterSavedGame.MasterSavedGame_C"))
        (Variables|Default|SetSaveGameData _returnvalue_2)
        (else
          (bind _returnvalue_3 (SaveGame|LoadGamefromSlot _savedgamename))
          (bind _asmaster_saved_game (Utilities|Casting|CastToMasterSavedGame _returnvalue_3))
          (Variables|Default|SetSaveGameData _asmaster_saved_game))))
    (:then_1
      (bind _returnvalue_4 (SaveGame|DoesSaveGameExist _inventorysavegamename))
      (if (not _returnvalue_4)
        (bind _returnvalue_5 (SaveGame|CreateSaveGameObject "/Game/Blueprints/SavingAndLoading/InventorySavedGame.InventorySavedGame_C"))
        (Variables|Default|SetInventorySaveGameData _returnvalue_5)
        (else
          (bind _returnvalue_6 (SaveGame|LoadGamefromSlot _inventorysavegamename))
          (bind _asinventory_saved_game (Utilities|Casting|CastToInventorySavedGame _returnvalue_6))
          (Variables|Default|SetInventorySaveGameData _asinventory_saved_game))))
    (:then_2
      (bind _returnvalue_7 (SaveGame|DoesSaveGameExist _levelsavegamename))
      (if (not _returnvalue_7)
        (bind _returnvalue_8 (SaveGame|CreateSaveGameObject "/Game/Blueprints/SavingAndLoading/LevelSavedGame.LevelSavedGame_C"))
        (Variables|Default|SetLevelSaveGameData _returnvalue_8)
        (else
          (bind _returnvalue_9 (SaveGame|LoadGamefromSlot _levelsavegamename))
          (bind _aslevel_saved_game (Utilities|Casting|CastToLevelSavedGame _returnvalue_9))
          (Variables|Default|SetLevelSaveGameData _aslevel_saved_game))))))

(fn SavePlayerData
  (bind _savegamedata (Variables|Default|GetSaveGameData))
  (bind _savedgamename (Variables|Default|GetSavedGameName))
  (bind _asplayer_character_bp (Utilities|Casting|CastToPlayerCharacter_BP (Game|GetPlayerCharacter 0)))
  (bind _output_get (Variables|Default|SetPlayerCharacterRef _asplayer_character_bp))
  (Utilities|FlowControl|Sequence
    (:then_0
      (bind _output_get_2 (Variables|/Game/Blueprints/SavingAndLoading/MasterSavedGame.MasterSavedGame_C|SetPlayer_Health _savegamedata (Variables|/Script/VoidSpoken.StatsMasterClass|GetHealth (Variables|/Script/VoidSpoken.BaseEntity|GetStats _output_get))))
      (Development|PrintString (Utilities|String|Append (Utilities|String|ToString(Float) _output_get_2) "Health Saved!")))
    (:then_1
      (bind _output_get_3 (Variables|/Game/Blueprints/SavingAndLoading/MasterSavedGame.MasterSavedGame_C|SetPlayer_Stamina _savegamedata (Variables|/Script/VoidSpoken.StatsMasterClass|GetStamina (Variables|/Script/VoidSpoken.BaseEntity|GetStats _output_get))))
      (Development|PrintString (Utilities|String|Append (Utilities|String|ToString(Float) _output_get_3) "Stamina Saved!")))
    (:then_2
      (bind _output_get_4 (Variables|/Game/Blueprints/SavingAndLoading/MasterSavedGame.MasterSavedGame_C|SetPlayer_Focus _savegamedata (Variables|/Script/VoidSpoken.StatsMasterClass|GetFocusPoints (Variables|/Script/VoidSpoken.BaseEntity|GetStats _output_get))))
      (Development|PrintString (Utilities|String|Append (Utilities|String|ToString(Float) _output_get_4) "Focus Saved!")))
    (:then_3
      (bind _output_get_5 (Variables|/Game/Blueprints/SavingAndLoading/MasterSavedGame.MasterSavedGame_C|SetPlayer_Location _savegamedata (Transformation|GetActorTransform (Variables|Default|GetPlayerCharacterRef))))
      (Development|PrintString (Utilities|String|Append (Utilities|String|ToString(Transform) _output_get_5) "Location Saved!"))))
  (bind _returnvalue (SaveGame|SaveGametoSlot (Variables|Default|GetSaveGameData) _savedgamename))
  (if _returnvalue
    (Development|PrintString (Utilities|String|Append "The Game has been saved to: " _savedgamename))
    (else
      (Development|PrintString "Failed to save!"))))

(fn LoadPlayerData
  (bind _savegamedata (Variables|Default|GetSaveGameData))
  (bind _asplayer_character_bp (Utilities|Casting|CastToPlayerCharacter_BP (Game|GetPlayerCharacter 0)))
  (bind _output_get (Variables|Default|SetPlayerCharacterRef _asplayer_character_bp))
  (Utilities|IsValid _output_get
    (:Is%20Valid
      (Utilities|FlowControl|Sequence
        (:then_0
          (bind _output_get_2 (Variables|/Script/VoidSpoken.StatsMasterClass|SetHealth (Variables|/Script/VoidSpoken.BaseEntity|GetStats _output_get) (Variables|/Game/Blueprints/SavingAndLoading/MasterSavedGame.MasterSavedGame_C|GetPlayer_Health _savegamedata)))
          (Development|PrintString (Utilities|String|Append (Utilities|String|ToString(Float) _output_get_2) "Health Loaded!")))
        (:then_1
          (bind _output_get_3 (Variables|/Script/VoidSpoken.StatsMasterClass|SetStamina (Variables|/Script/VoidSpoken.BaseEntity|GetStats _output_get) (Variables|/Game/Blueprints/SavingAndLoading/MasterSavedGame.MasterSavedGame_C|GetPlayer_Stamina _savegamedata)))
          (Development|PrintString (Utilities|String|Append (Utilities|String|ToString(Float) _output_get_3) "Stamina Loaded")))
        (:then_2
          (bind _output_get_4 (Variables|/Script/VoidSpoken.StatsMasterClass|SetFocusPoints (Variables|/Script/VoidSpoken.BaseEntity|GetStats _output_get) (Variables|/Game/Blueprints/SavingAndLoading/MasterSavedGame.MasterSavedGame_C|GetPlayer_Focus _savegamedata)))
          (Development|PrintString (Utilities|String|Append (Utilities|String|ToString(Float) _output_get_4) "Focus Loaded")))
        (:then_3
          (bind _output_get_5 (Variables|/Game/Blueprints/Player/PlayerCharacter_BP.PlayerCharacter_BP_C|SetPlayerLocation _output_get (Variables|/Game/Blueprints/SavingAndLoading/MasterSavedGame.MasterSavedGame_C|GetPlayer_Location _savegamedata)))
          (Development|PrintString (Utilities|String|Append (Utilities|String|ToString(Transform) _output_get_5) "Loaded!"))
          (Transformation|SetActorLocation (Variables|Default|GetPlayerCharacterRef) (.Location (Math|Transform|BreakTransform _output_get_5)) false false))))))

(fn SaveInventoryData
  (params (PlayerCharacter :type Player%20Character%20BP%20Object%20Reference))
  (bind _inventorysavegamename (Variables|Default|GetInventorySaveGameName))
  (bind _inventorysavegamedata (Variables|Default|GetInventorySaveGameData)
    (:then
      (bind _output_get (Variables|/Game/Blueprints/SavingAndLoading/InventorySavedGame.InventorySavedGame_C|SetPlayer_InventoryData _inventorysavegamedata (Variables|/Game/Blueprints/SavingAndLoading/InventorySaving/InventoryComponent.InventoryComponent_C|GetInventoryContent (Variables|/Game/Blueprints/Player/PlayerCharacter_BP.PlayerCharacter_BP_C|GetInventory%20Component PlayerCharacter))))
      (Utilities|FlowControl|Sequence
        (:then_0
          (bind _returnvalue (SaveGame|SaveGametoSlot _inventorysavegamedata _inventorysavegamename))
          (if _returnvalue
            (Development|PrintString (Utilities|String|Append "The Game has been saved to: " _inventorysavegamename))
            (else
              (Development|PrintString "Failed to save!"))))
        (:then_1
          (Development|PrintString (Utilities|String|Append "Collected Healing Pickup: " (Utilities|String|ToString(Integer) (.Value (Utilities|Map|Find _output_get "HealingPickup"))) " (Saved)") true true "(R=1.000000,G=0.936081,B=0.000000,A=1.000000)")
          (Development|PrintString (Utilities|String|Append "Collected Focus Pickup: " (Utilities|String|ToString(Integer) (.Value (Utilities|Map|Find _output_get "FocusPickup"))) " (Saved)") true true "(R=1.000000,G=0.936081,B=0.000000,A=1.000000)")
          (Development|PrintString (Utilities|String|Append "Collected Stamina Pickup:  " (Utilities|String|ToString(Integer) (.Value (Utilities|Map|Find _output_get "StaminaPickup"))) " (Saved)") true true "(R=1.000000,G=0.936081,B=0.000000,A=1.000000)"))))
    (:else)))

(fn LoadInventoryData
  (params (PlayerCharacter :type Player%20Character%20BP%20Object%20Reference))
  (bind _inventorysavegamedata (Variables|Default|GetInventorySaveGameData))
  (bind _player_inventorydata (Variables|/Game/Blueprints/SavingAndLoading/InventorySavedGame.InventorySavedGame_C|GetPlayer_InventoryData _inventorysavegamedata))
  (Variables|/Game/Blueprints/SavingAndLoading/InventorySaving/InventoryComponent.InventoryComponent_C|SetInventoryContent (Variables|/Game/Blueprints/Player/PlayerCharacter_BP.PlayerCharacter_BP_C|GetInventory%20Component PlayerCharacter) _player_inventorydata)
  (Development|PrintString (Utilities|String|Append "Collected Stamina Pickup:  " (Utilities|String|ToString(Integer) (.Value (Utilities|Map|Find _player_inventorydata "StaminaPickup"))) " (Loaded)") true true "(R=1.000000,G=0.871116,B=0.000000,A=1.000000)")
  (Development|PrintString (Utilities|String|Append "Collected Focus Pickup: " (Utilities|String|ToString(Integer) (.Value (Utilities|Map|Find _player_inventorydata "FocusPickup"))) " (Loaded)") true true "(R=1.000000,G=0.871116,B=0.000000,A=1.000000)")
  (Development|PrintString (Utilities|String|Append "Collected Healing Pickup: " (Utilities|String|ToString(Integer) (.Value (Utilities|Map|Find _player_inventorydata "HealingPickup"))) " (Loaded)") true true "(R=1.000000,G=0.871116,B=0.000000,A=1.000000)"))