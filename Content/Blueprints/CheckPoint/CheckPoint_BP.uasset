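; Checkpoint actor that activates linked enemy spawners and saves player data when the player walks into it.
; On BeginPlay it caches the VoidSpokenGameInstance.
; Its collision overlap filters for player pawn 0, then sends an activate message to each entry in ActivateSpawn before calling SavePlayerData on the game instance.
; Nothing in the overlap limits it to a single use, so each re-entry repeats both steps.
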(event OnComponentBeginOverlap(CheckpointMeshCollision)
  (params (OverlappedComponent :type Primitive%20Component%20Object%20Reference) (OtherActor :type Actor%20Object%20Reference) (OtherComp :type Primitive%20Component%20Object%20Reference) (OtherBodyIndex :type Integer) (bFromSweep :type Boolean) (SweepResult :type Hit%20Result%20Structure%20%28by%20ref%29))
  (if (== (Game|Player|GetPlayerPawn 0) OtherActor)
    (Utilities|FlowControl|Sequence
      (:then_0
        ;[0 0 0] Spawn Enemy
        (for _array_element (Variables|Default|GetActivateSpawn)
          (Class|ActivateSpawnBPI|ActivateEnemySpawner(Message) _array_element)))
      (:then_1
        ;[0 0 0] Saves Player's Data
        (Default|SavePlayerData (Variables|Default|GetGameInstanceRef))))))

(event EventBeginPlay
  (bind _asvoid_spoken_game_instance (Utilities|Casting|CastToVoidSpokenGameInstance (Game|GetGameInstance)))
  (Variables|Default|SetGameInstanceRef _asvoid_spoken_game_instance))

(fn ConstructionScript)