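; Music manager that plays menu, combat and out-of-combat ambiance tracks.
; On BeginPlay it binds to start and end combat events to switch between combat and ambiance music.
; Each play function sets CurrentTrack, starts it with fire-and-forget PlaySound2D and prints a debug string.
; Nothing stops a playing sound, so tracks can overlap; StopMusic only clears CurrentTrack.
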(event Custom|Start%20CombatMusic
  (CallFunction|PlayCombatMusic))

(event Custom|End%20Combat%20Music
  (CallFunction|PlayAmbianceMusic))

(event EventBeginPlay
  (EventDispatchers|BindEventtoStartCombat (delegate Custom|Start%20CombatMusic))
  (EventDispatchers|BindEventtoEndCombat (delegate Custom|End%20Combat%20Music)))

(fn ConstructionScript)

(fn PlayMenuMusic
  (bind _output_get (Variables|Default|SetCurrentTrack (Variables|Default|GetMain%20menu%20music)))
  (Audio|PlaySound2D _output_get 1.0 1.0 0.0 0 0)
  (Development|PrintString "MainMenu"))

(fn PlayCombatMusic
  (bind _output_get (Variables|Default|SetCurrentTrack (Variables|Default|GetCombat%20music)))
  (Audio|PlaySound2D _output_get 1.0 1.0 0.0 0 0)
  (Development|PrintString "playing combat"))

(fn PlayAmbianceMusic
  (bind _output_get (Variables|Default|SetCurrentTrack (Variables|Default|Getout%20of%20combat%20music)))
  (Audio|PlaySound2D _output_get 1.0 1.0 0.0 0 0)
  (Development|PrintString "Ambiance"))

(fn StopMusic
  (Variables|Default|SetCurrentTrack 0))