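; Outdoor wind ambience actor that starts its sound when the player character enters a trigger box.
; The construction script applies the exposed sound cue, attenuation, volume multiplier and box extent to the audio and collision components.
; Box overlap casts to PlayerCharacter_BP and plays the sound from the beginning, with no logic to stop it on exit.
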(event OnComponentBeginOverlap(BoxCollision)
  (params (OverlappedComponent :type Primitive%20Component%20Object%20Reference) (OtherActor :type Actor%20Object%20Reference) (OtherComp :type Primitive%20Component%20Object%20Reference) (OtherBodyIndex :type Integer) (bFromSweep :type Boolean) (SweepResult :type Hit%20Result%20Structure%20%28by%20ref%29))
  (Utilities|Casting|CastToPlayerCharacter_BP OtherActor)
  (Audio|Components|Audio|Play (Variables|Default|GetAmbientSound) 0.0))

(event EventBeginPlay)

(event Collision|EventActorBeginOverlap
  (params (OtherActor :type Actor%20Object%20Reference)))

(event EventTick
  (params (DeltaSeconds :type Float%20%28single-precision%29)))

(fn ConstructionScript
  (bind _ambientsound (Variables|Default|GetAmbientSound))
  (Audio|Components|Audio|SetSound (Variables|Default|GetAmbientSound) (Variables|Default|GetSoundCue))
  (Variables|/Script/Engine.AudioComponent|SetAttenuationSettings _ambientsound (Variables|Default|GetAmbientSoundAttenuation))
  (Audio|Components|Audio|SetVolumeMultiplier _ambientsound (Variables|Default|GetVolumeMultiplier) :!class /Script/Engine.AudioComponent)
  (Components|Box|SetBoxExtent (Variables|Default|GetBoxCollision) (Variables|Default|GetBoxSize) true))