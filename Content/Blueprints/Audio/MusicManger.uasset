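; Music manager actor that plays one 2D music track at a time and switches between combat and ambiance music.
; BeginPlay starts CurrentTrack through StartMusic, which destroys any still-playing player, spawns a new 2D sound and stores it in Player1.
; The switch functions print a debug message, stop any playing track, set CurrentTrack and restart with no explicit crossfade.
; StopMusic stops the current player.
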(event EventBeginPlay
  (CallFunction|StartMusic))

(event Collision|EventActorBeginOverlap
  (params (OtherActor :type Actor%20Object%20Reference)))

(event EventTick
  (params (DeltaSeconds :type Float%20%28single-precision%29)))

(fn ConstructionScript)

(fn SwitchtoCombatMusic
  (bind _player1 (Variables|Default|GetPlayer1))
  (Development|PrintString "switching to combat")
  (if (Audio|Components|Audio|IsPlaying _player1)
    (Audio|Components|Audio|Stop _player1)
    (Variables|Default|SetCurrent%20track (Variables|Default|GetCombat%20music))
    (CallFunction|StartMusic)
    (else
      (Variables|Default|SetCurrent%20track (Variables|Default|GetCombat%20music))
      (CallFunction|StartMusic))))

(fn SwitchtoAmbianceMusic
  (bind _player1 (Variables|Default|GetPlayer1))
  (Development|PrintString "switching to ambiance")
  (if (Audio|Components|Audio|IsPlaying _player1)
    (Audio|Components|Audio|Stop _player1)
    (Variables|Default|SetCurrent%20track (Variables|Default|GetAmbiance%20music))
    (CallFunction|StartMusic)
    (else
      (Variables|Default|SetCurrent%20track (Variables|Default|GetAmbiance%20music))
      (CallFunction|StartMusic))))

(fn StopMusic
  (Audio|Components|Audio|Stop (Variables|Default|GetPlayer1)))

(fn StartMusic
  (if (Audio|Components|Audio|IsPlaying (Variables|Default|GetPlayer1))
    (Components|DestroyComponent (Variables|Default|GetPlayer1)))
  (bind _returnvalue (Audio|SpawnSound2D (Variables|Default|GetCurrent%20track) 1.0 1.0 0.0 0))
  (Variables|Default|SetPlayer1 _returnvalue))