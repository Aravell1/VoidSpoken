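; AudioTrigger is a trigger volume actor that plays an audio track when the player character overlaps its Box.
; AudioTrackType selects playback: voice lines and music play in 2D, while SFX can play at the Sphere's location.
; DestroyOnceTouched removes the actor only after a located SFX plays.
; PlayOnlyOnce leads into a DoOnce whose output triggers nothing.
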(event OnComponentBeginOverlap(Box)
  (params (OverlappedComponent :type Primitive%20Component%20Object%20Reference) (OtherActor :type Actor%20Object%20Reference) (OtherComp :type Primitive%20Component%20Object%20Reference) (OtherBodyIndex :type Integer) (bFromSweep :type Boolean) (SweepResult :type Hit%20Result%20Structure%20%28by%20ref%29))
  (bind _audiotrack (Variables|Default|GetAudioTrack))
  (bind _audiotrack_2 (Variables|Default|GetAudioTrack))
  (if (== OtherActor (Game|GetPlayerCharacter 0))
    (if (Variables|Default|GetPlay%20only%20once)
      (Utilities|FlowControl|DoOnce false
        (:Completed
          _)))
    (switch Utilities|FlowControl|Switch|SwitchonTrackType (Variables|Default|GetAudioTrackType)
      (:NewEnumerator0
        (Audio|PlaySound2D _audiotrack_2 1.0 1.0 0.0 0 0))
      (:NewEnumerator1
        (Audio|PlaySound2D _audiotrack_2 1.0 1.0 0.0 0 0))
      (:NewEnumerator2
        (if (Variables|Default|GetPlayAtLocation)
          (Audio|PlaySoundatLocation _audiotrack (Transformation|GetWorldLocation (Variables|Default|GetSphere)) "0, 0, 0" 1.0 1.0 0.0 0 0 0 0)
          (if (Variables|Default|GetDestroyOnceTouched)
            (Actor|DestroyActor))
          (else
            (Audio|PlaySound2D _audiotrack 1.0 1.0 0.0 0 0)))))))

(event EventBeginPlay)

(event Collision|EventActorBeginOverlap
  (params (OtherActor :type Actor%20Object%20Reference)))

(event EventTick
  (params (DeltaSeconds :type Float%20%28single-precision%29)))

(fn ConstructionScript)