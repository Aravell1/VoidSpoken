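; Base enemy AI that patrols, chases a spotted player and makes melee attacks.
; BehaviourUnit re-calls itself as a state machine, alternating random roaming with visits to the nearest patrol point until PawnSensing switches it to chase.
; On arrival, a DoOnce-gated montage plays while the enemy turns toward the player, and its notify fires a damaging sphere trace.
; A failed chase move reverts to roaming if the target is too far.
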(event OnSeePawn(PawnSensing)
  (params (Pawn :type Pawn%20Object%20Reference))
  ;[1 1 1] Chases the player if spotted
  (if (not (Variables|Default|GetDead?))
    (Variables|/Script/Engine.CharacterMovementComponent|SetMaxWalkSpeed (Variables|Character|GetCharacterMovement) 4.5e+02)
    (bind _asmy_character (Utilities|Casting|CastToTemp_PlayerCharacter Pawn))
    (Variables|Default|SetAttackTarget _asmy_character)
    (Variables|Default|SetBehaviourMode "NewEnumerator2")
    (CallFunction|BehaviourUnit)))

(event Custom|BehaviourUnit
  (bind _charactermovement (Variables|Character|GetCharacterMovement))
  (if (not (Variables|Default|GetDead?))
    (switch Utilities|FlowControl|Switch|SwitchonBehaviourModes (Variables|Default|GetBehaviourMode)
      (:NewEnumerator0
        (Variables|/Script/Engine.CharacterMovementComponent|SetMaxWalkSpeed (Variables|Character|GetCharacterMovement) 225.0)
        (AI|AIMoveTo self (.RandomLocation (AI|Navigation|GetRandomReachablePointinRadius (Transformation|GetActorLocation) (Variables|Default|GetRoamRadius) 0 0)) 0 5.0 false
          (:then
            (CallFunction|UpdatePatrolPoint)
            (Utilities|FlowControl|Delay (Math|Random|RandomFloatinRange (Variables|Default|GetMinWait) (Variables|Default|GetMaxWait)))
            (if (Utilities|Enum|Equal(Enum) (Variables|Default|GetBehaviourMode) "NewEnumerator2")
              (CallFunction|ChasePlayer :!label _label)
              (else
                (Variables|Default|SetBehaviourMode "NewEnumerator1")
                (CallFunction|BehaviourUnit))))))
      (:NewEnumerator1
        (Variables|/Script/Engine.CharacterMovementComponent|SetMaxWalkSpeed (Variables|Character|GetCharacterMovement) 225.0)
        (AI|AIMoveTo self "0, 0, 0" (Variables|Default|GetPatrolPointRef) 5.0 false
          (:OnSuccess
            (Utilities|FlowControl|Delay (Math|Random|RandomFloatinRange (Variables|Default|GetMinWait) (Variables|Default|GetMaxWait)))
            (if (Utilities|Enum|Equal(Enum) (Variables|Default|GetBehaviourMode) "NewEnumerator2")
              (goto _label)
              (else
                (Variables|Default|SetBehaviourMode "NewEnumerator0")
                (CallFunction|BehaviourUnit))))))
      (:NewEnumerator2
        (if (not (Variables|Default|GetDead?))
          (AI|AIMoveTo self "0, 0, 0" (Variables|Default|GetAttackTarget) (Variables|Default|GetAttackAcceptanceRadius) false
            (:OnSuccess
              (Utilities|FlowControl|DoOnce false
                (:Completed
                  (Variables|Default|SetAttackingPlayer? true)
                  (bind _notifyname (Animation|Montage|PlayMontage (Variables|Character|GetMesh) (Variables|Default|GetAttackMontage))
                    (:then
                      (Components|Movement|StopMovementImmediately _charactermovement)
                      (Variables|/Script/Engine.CharacterMovementComponent|SetMaxWalkSpeed _charactermovement 0.0)
                      (CallFunction|TrackPlayer))
                    (:OnCompleted
                      (Utilities|FlowControl|Delay (Math|Random|RandomFloatinRange 0.1 0.3))
                      (Variables|Default|SetAttackingPlayer? false)
                      (if (not (Variables|Default|GetDead?))
                        (CallFunction|ReleaseAttack)
                        (Variables|/Script/Engine.CharacterMovementComponent|SetMaxWalkSpeed (Variables|Character|GetCharacterMovement) 4.5e+02)
                        (CallFunction|BehaviourUnit)))
                    (:OnNotifyBegin
                      (switch name _notifyname
                        (:AttackTrace
                          (CallFunction|AttackTrace))))))))
            (:OnFail
              (CallFunction|ChaseDistanceCheck))))))))

(event Custom|ChasePlayer
  (bind _charactermovement (Variables|Character|GetCharacterMovement))
  (if (not (Variables|Default|GetDead?))
    (AI|AIMoveTo self "0, 0, 0" (Variables|Default|GetAttackTarget) (Variables|Default|GetAttackAcceptanceRadius) false
      (:OnSuccess
        (Utilities|FlowControl|DoOnce false
          (:Completed
            (Variables|Default|SetAttackingPlayer? true)
            (bind _notifyname (Animation|Montage|PlayMontage (Variables|Character|GetMesh) (Variables|Default|GetAttackMontage))
              (:then
                (Components|Movement|StopMovementImmediately _charactermovement)
                (Variables|/Script/Engine.CharacterMovementComponent|SetMaxWalkSpeed _charactermovement 0.0)
                (CallFunction|TrackPlayer))
              (:OnCompleted
                (Utilities|FlowControl|Delay (Math|Random|RandomFloatinRange 0.1 0.3))
                (Variables|Default|SetAttackingPlayer? false)
                (if (not (Variables|Default|GetDead?))
                  (CallFunction|ReleaseAttack)
                  (Variables|/Script/Engine.CharacterMovementComponent|SetMaxWalkSpeed (Variables|Character|GetCharacterMovement) 4.5e+02)
                  (CallFunction|BehaviourUnit)))
              (:OnNotifyBegin
                (switch name _notifyname
                  (:AttackTrace
                    (CallFunction|AttackTrace))))))))
      (:OnFail
        (CallFunction|ChaseDistanceCheck)))))

(event Custom|ReleaseAttack
  (bind _charactermovement (Variables|Character|GetCharacterMovement))
  (Utilities|FlowControl|DoOnce false) ; enters at Reset
)

(event Custom|TrackPlayer
  ;[1 1 1] Rotates toward the player while attacking
  (Variables|Default|GetAttackTarget
    (:then
      (if (Variables|Default|GetAttackingPlayer?)
        (Transformation|SetActorRotation (Math|Rotator|MakeRotator 0.0 0.0 (.yaw (Math|Rotator|FindLookatRotation (Transformation|GetActorLocation) (Transformation|GetActorLocation (Variables|Default|GetAttackTarget))))))
        (Utilities|FlowControl|Delay 0.01)
        (CallFunction|TrackPlayer)))
    (:else)))

(event Custom|ChaseDistanceCheck
  ;[1 1 1] Stops chasing if the player is out of range
  (if (not (Variables|Default|GetDead?))
    (if (> (Math|Vector|Distance(Vector) (Transformation|GetActorLocation) (Transformation|GetActorLocation (Variables|Default|GetAttackTarget))) 2.5e+03)
      (Variables|Default|SetBehaviourMode "NewEnumerator0")
      (CallFunction|BehaviourUnit))))

(event EventBeginPlay
  (CallFunction|BehaviourUnit))

(fn ConstructionScript
  (bind _self self)
  (bind _outactors (Actor|GetAllActorsOfClass "/Game/Enemies/EnemyPatrolPoint_BP.EnemyPatrolPoint_BP_C"))
  (Variables|Default|SetPatrolPointRef (Utilities|Array|Get(acopy) _outactors))
  (for _array_element _outactors
    (if (< (Transformation|GetDistanceTo _array_element _self) (Transformation|GetDistanceTo (Variables|Default|GetPatrolPointRef) _self))
      (Variables|Default|SetPatrolPointRef _array_element))))

(fn UpdatePatrolPoint
  (bind _self self)
  (bind _outactors (Actor|GetAllActorsOfClass "/Game/Enemies/EnemyPatrolPoint_BP.EnemyPatrolPoint_BP_C"))
  (for _array_element _outactors
    (if (< (Transformation|GetDistanceTo _array_element _self) (Transformation|GetDistanceTo (Variables|Default|GetPatrolPointRef) _self))
      (Variables|Default|SetPatrolPointRef _array_element))))

(fn AttackTrace
  (bind _returnvalue (Transformation|GetActorLocation))
  (bind _attack_dmg (Variables|Default|GetAttack%20DMG))
  (bind (_outhit _returnvalue_2) (Collision|SphereTraceByChannel _returnvalue (+ _returnvalue (* (Transformation|GetActorForwardVector) (Variables|Default|GetAttackRange))) (Variables|Default|GetAttackRadius) "TraceTypeQuery1" false 0 "ForDuration"))
  (if _returnvalue_2
    (Game|Damage|ApplyDamage (.HitActor (Collision|BreakHitResult _outhit)) (Math|Conversions|ToFloat(Integer) (Math|Float|Round (Math|Random|RandomFloatinRange (Math|Conversions|ToFloat(Integer) (- _attack_dmg 2)) (Math|Conversions|ToFloat(Integer) (+ _attack_dmg 2))))) 0 0)))